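; Debug damage meter that records damage taken by the player and counts spawned projectiles.
; Arrancar resets the totals, snapshots player stats from BP_StatsManagerComponent and starts a looping timer on Muestrear.
; Each sample adds any health drop to the total, merging consecutive drops into one hit and logging intervals between hits.
; ContarFlechas infers new arrows from increases in the live projectile actor count and timestamps them.
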(fn `Arrancar`
  ; Comment
  (set `self.UltimaVida` (`.BaseValue_2_4D90BE9B410B9CC673FEFCB292CBF2BC` (break `/Game/DynamicCombatSystem/DCS/Blueprints/Components/StatsManager/F_Stat` (`|GetArrayItem` (`/Game/DynamicCombatSystem/DCS/Blueprints/Components/StatsManager/BP_StatsManagerComponent.Stats` (`self.GetComponentByClass` (`GameplayStatics.GetPlayerCharacter` 0) "/Game/DynamicCombatSystem/DCS/Blueprints/Components/StatsManager/BP_StatsManagerComponent.BP_StatsManagerComponent_C")) (`self.IndiceVida`)))))
  (set `self.UltimosGolpes` (`.BaseValue_2_4D90BE9B410B9CC673FEFCB292CBF2BC` (break `/Game/DynamicCombatSystem/DCS/Blueprints/Components/StatsManager/F_Stat` (`|GetArrayItem` (`/Game/DynamicCombatSystem/DCS/Blueprints/Components/StatsManager/BP_StatsManagerComponent.Stats` (`self.GetComponentByClass` (`GameplayStatics.GetPlayerCharacter` 0) "/Game/DynamicCombatSystem/DCS/Blueprints/Components/StatsManager/BP_StatsManagerComponent.BP_StatsManagerComponent_C")) (`self.IndiceGolpes`)))))
  (set `self.Golpes` 0.0)
  (set `self.EnGolpe` false)
  (set `self.DanoTotal` 0.0)
  (`KismetArrayLibrary.Array_Clear` (`self.Intervalos`))
  (set `self.Flechas` 0)
  (set `self.UltimasFlechas` 0)
  (`KismetArrayLibrary.Array_Clear` (`self.TiemposFlecha`))
  (set `self.TInicio` (`KismetSystemLibrary.GetGameTimeInSeconds`))
  (set `self.TUltimoGolpe` (`KismetSystemLibrary.GetGameTimeInSeconds`))
  (set `self.Midiendo` true)
  (`KismetSystemLibrary.K2_SetTimer` self "Muestrear" (`self.Intervalo`) true))

(fn `ContarFlechas`
  (bind _ultimasflechas (`self.UltimasFlechas`))
  ; Comment
  ;; Comment
  (bind _outactors (`GameplayStatics.GetAllActorsOfClass` (`self.ClaseProyectil`)))
  (bind _returnvalue (`KismetArrayLibrary.Array_Length` _outactors))
  ; Comment
  ;; Comment
  (if (> _returnvalue _ultimasflechas)
    (set `self.Flechas` (+ (`self.Flechas`) (- _returnvalue _ultimasflechas)))
    (`KismetArrayLibrary.Array_Add` (`self.TiemposFlecha`) (- (`KismetSystemLibrary.GetGameTimeInSeconds`) (`self.TInicio`))))
  ; Comment
  (set `self.UltimasFlechas` _returnvalue))

(fn `Muestrear`
  (bind (_attributetag _basevalue) (break `/Game/DynamicCombatSystem/DCS/Blueprints/Components/StatsManager/F_Stat` (`|GetArrayItem` (`/Game/DynamicCombatSystem/DCS/Blueprints/Components/StatsManager/BP_StatsManagerComponent.Stats` (`self.GetComponentByClass` (`GameplayStatics.GetPlayerCharacter` 0) "/Game/DynamicCombatSystem/DCS/Blueprints/Components/StatsManager/BP_StatsManagerComponent.BP_StatsManagerComponent_C")) (`self.IndiceVida`))))
  (bind _returnvalue (- (`self.UltimaVida`) _basevalue))
  (if (`self.Midiendo`)
    (`self.ContarFlechas`)
    (if (> _returnvalue 0.0)
      (set `self.DanoTotal` (+ (`self.DanoTotal`) _returnvalue))
      (if (not (`self.EnGolpe`))
        (set `self.Golpes` (+ (`self.Golpes`) 1.0))
        (`KismetArrayLibrary.Array_Add` (`self.Intervalos`) (- (`KismetSystemLibrary.GetGameTimeInSeconds`) (`self.TUltimoGolpe`)))
        (set `self.TUltimoGolpe` (`KismetSystemLibrary.GetGameTimeInSeconds`))
        (set `self.EnGolpe` true))
      (else
        (set `self.EnGolpe` false)))
    (set `self.UltimaVida` _basevalue)))

(fn `UserConstructionScript`)

(fn `ZZProbeMedidor`)