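; Mirror threshold that shows a live reflection and works as a one-shot teleport.
; Each tick Reflejo, a scene capture, mirrors the player's view across the plane of Espejo, whose dynamic material receives the Imagen texture.
; When a BP_CombatCharacter overlaps while active, the glass switches to a broken material, capture stops and the player teleports to Destino, facing the threshold.
; OcultarDetras hides the mirror and static meshes behind it from capture, but is not called here.
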(event `self.ReceiveActorBeginOverlap`
  (params (OtherActor :type "Actor Object Reference"))
  (if (`self.Activo`)
    (bind _asbp_combat_character (cast `/Game/DynamicCombatSystem/DCS/Blueprints/BP_CombatCharacter` OtherActor))
    (`/Engine/EditorBlueprintResources/StandardMacros.IsValid` _asbp_combat_character
      (:`Is Valid`
        (set `self.Activo` false)
        (`self.RomperEspejo`)
        (`self.Cruzar`)))))

(event `self.ReceiveTick`
  (params (DeltaSeconds :type "Float (single-precision)"))
  (`self.ActualizarReflejo`))

(event `self.ReceiveBeginPlay`
  (`self.Encender`))

(fn `ActualizarReflejo`
  (bind (_location _rotation) (`Controller.GetPlayerViewPoint` (`GameplayStatics.GetPlayerController` 0)))
  (bind _returnvalue (`self.K2_GetActorLocation` (`self.Espejo`)))
  (bind _returnvalue_2 (`KismetMathLibrary.GetForwardVector` _rotation))
  (bind _returnvalue_3 (`KismetMathLibrary.Vector_NormalUnsafe` (- (`self.K2_GetActorLocation` self) _returnvalue)))
  (if (`self.Vivo`)
    (`SceneComponent.K2_SetWorldLocationAndRotation` (`self.Reflejo`) (- _location (* _returnvalue_3 (* 2.0 (`KismetMathLibrary.Dot_VectorVector` (- _location _returnvalue) _returnvalue_3)))) (`KismetMathLibrary.MakeRotFromX` (- _returnvalue_2 (* _returnvalue_3 (* 2.0 (`KismetMathLibrary.Dot_VectorVector` _returnvalue_2 _returnvalue_3))))) false true)))

(fn `Cruzar`
  (bind _destino (`self.Destino`))
  (bind _returnvalue (`self.K2_GetActorLocation` _destino))
  (bind _returnvalue_2 (`KismetMathLibrary.MakeRotator` 0.0 0.0 (.yaw (`KismetMathLibrary.FindLookAtRotation` _returnvalue (`self.K2_GetActorLocation` self)))))
  (`/Engine/EditorBlueprintResources/StandardMacros.IsValid` _destino
    (:`Is Valid`
      (`self.K2_SetActorLocationAndRotation` (`GameplayStatics.GetPlayerPawn` 0) _returnvalue _returnvalue_2 false true)
      (`Controller.SetControlRotation` (`GameplayStatics.GetPlayerController` 0) _returnvalue_2))))

(fn `Encender`
  (bind _returnvalue (`self.GetComponentByClass` (`self.Espejo`) "/Script/Engine.StaticMeshComponent"))
  (`/Engine/EditorBlueprintResources/StandardMacros.IsValid` _returnvalue
    (:`Is Valid`
      (bind _returnvalue_2 (`PrimitiveComponent.CreateDynamicMaterialInstance` _returnvalue 0 "/Game/DarkAngels/Materials/Malkuth/M_DA_MK_Espejo_Imagen.M_DA_MK_Espejo_Imagen" "None"))
      (`MaterialInstanceDynamic.SetTextureParameterValue` _returnvalue_2 "Imagen" (`self.Imagen`)))))

(fn `OcultarDetras`
  (bind _espejo (`self.Espejo`))
  (bind _reflejo (`self.Reflejo`))
  (bind _returnvalue (`self.K2_GetActorLocation` _espejo))
  (`SceneCaptureComponent.HideActorComponents` _reflejo _espejo true)
  (bind _outactors (`GameplayStatics.GetAllActorsOfClass` "/Script/Engine.StaticMeshActor"))
  (for _array_element _outactors
    (if (< (`KismetMathLibrary.Dot_VectorVector` (- (`self.K2_GetActorLocation` _array_element) _returnvalue) (`KismetMathLibrary.Vector_NormalUnsafe` (- (`self.K2_GetActorLocation` self) _returnvalue))) -20.0)
      (`SceneCaptureComponent.HideActorComponents` _reflejo _array_element true))))

(fn `RomperEspejo`
  (bind _returnvalue (`self.GetComponentByClass` (`self.Espejo`) "/Script/Engine.StaticMeshComponent"))
  (set `self.Vivo` false)
  (set `SceneCaptureComponent.bCaptureEveryFrame` false (`self.Reflejo`))
  (`/Engine/EditorBlueprintResources/StandardMacros.IsValid` _returnvalue
    (:`Is Valid`
      (`PrimitiveComponent.SetMaterial` _returnvalue 0 "/Game/DarkAngels/Materials/Malkuth/M_DA_MK_Espejo_Roto.M_DA_MK_Espejo_Roto"))))

(fn `UserConstructionScript`)