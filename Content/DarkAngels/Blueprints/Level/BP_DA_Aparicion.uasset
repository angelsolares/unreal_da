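; Level actor that makes a set of target actors appear or vanish with a dissolve once a game-state requirement is met.
; If set to appear, it dissolves the targets out and disables their collision on BeginPlay.
; Tick polls BP_DA_GameState for the requirement, then fires once, marking a flag and switching collision.
; The Disolver component dissolves each target mesh, reversed for appearing.
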(event `self.ReceiveBeginPlay`
  (if (`self.Aparecer`)
    (`self.AplicarDisolver` false)))

(event `self.ReceiveTick`
  (params (DeltaSeconds :type "Float (single-precision)"))
  (`self.VigilarAparicion`))

(fn `AplicarDisolver`
  (params (Mostrar :type Boolean))
  (set `/Game/DynamicCombatSystem/DCS/Blueprints/Components/Dissolve/BP_DissolveComponent.DissolveColor` (make `LinearColor` 5.0 3.2 1.2 0.0) (`self.Disolver`))
  (for _array_element (`self.Objetivos`)
    (`self.SetActorEnableCollision` _array_element Mostrar)
    (for _array_element_2 (`self.K2_GetComponentsByClass` _array_element "/Script/Engine.MeshComponent")
      (bind _asprimitive_component (cast `PrimitiveComponent` _array_element_2))
      (`/Game/DynamicCombatSystem/DCS/Blueprints/Components/Dissolve/BP_DissolveComponent.StartDissolve` (`self.Disolver`) _asprimitive_component Mostrar))))

(fn `UserConstructionScript`)

(fn `VigilarAparicion`
  (bind _asbp_da_game_state (cast `/Game/DarkAngels/Blueprints/World/BP_DA_GameState` (`GameplayStatics.GetGameState`)))
  (bind _tiene (`/Game/DarkAngels/Blueprints/World/BP_DA_GameState.Lleva` _asbp_da_game_state (`self.Requisito`)))
  (if (and (not (`self.Hecho`)) (and (not (`KismetStringLibrary.IsEmpty` (`self.Requisito`))) _tiene))
    (set `self.Hecho` true)
    (`/Game/DarkAngels/Blueprints/World/BP_DA_GameState.MarcarFlag` _asbp_da_game_state (`self.FlagAlPasar`))
    (`self.AplicarDisolver` (`self.Aparecer`))))