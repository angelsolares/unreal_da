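; Glowing light actor (Fuego) that travels along a route of points: warm and bright when Principal, cool and dimmer otherwise.
; Once Listo, Tick snaps its index to the nearest Ruta point, destroying itself if that is beyond Radio.
; It then flies straight point to point at a height offset, advancing within Cerca and destroying itself at the end.
; A fixed lifespan caps it; several disconnected older Tick copies remain unused.
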(event `self.ReceiveBeginPlay`
  (`self.SetLifeSpan` self 14.0)
  (if (`self.Principal`)
    (`LightComponent.SetLightColor` (`self.Luz`) (struct :`R` 1.0 :`G` 0.78 :`B` 0.36 :`A` 1.0) false)
    (`LightComponent.SetIntensity` (`self.Luz`) 90000.0)
    (else
      (`LightComponent.SetLightColor` (`self.Luz`) (struct :`R` 0.42 :`G` 0.55 :`B` 0.85 :`A` 1.0) false)
      (`LightComponent.SetIntensity` (`self.Luz`) 35000.0))))

(event `self.ReceiveTick`
  (params (DeltaSeconds :type "Float (single-precision)"))
  (bind _returnvalue (`self.K2_GetActorLocation` self))
  (bind _puntos (`/Game/DarkAngels/Blueprints/Level/BP_DA_Ruta.Puntos` (`self.Ruta`)))
  (bind _returnvalue_2 (+ (`|GetArrayItem` _puntos (`self.Indice`)) (`KismetMathLibrary.MakeVector` 0.0 0.0 (`self.Altura`))))
  (if (`self.Listo`)
    (if (< (`self.Indice`) 0)
      (set `self.MejorDist` 100000000.0)
      (for _index (range (+ (- (`KismetArrayLibrary.Array_Length` _puntos) 1) 1))
        (if (< (`KismetMathLibrary.Vector_Distance` (`|GetArrayItem` _puntos _index) (`self.K2_GetActorLocation` self)) (`self.MejorDist`))
          (set `self.MejorDist` (`KismetMathLibrary.Vector_Distance` (`|GetArrayItem` _puntos _index) (`self.K2_GetActorLocation` self)))
          (set `self.Indice` _index)))
      (if (> (`self.MejorDist`) (`self.Radio`))
        (`self.K2_DestroyActor` self))
      (elif (>= (`self.Indice`) (`KismetArrayLibrary.Array_Length` _puntos))
        (`self.K2_DestroyActor` self)
        (else
          (`self.K2_SetActorLocation` self (+ _returnvalue (* (`KismetMathLibrary.GetDirectionUnitVector` _returnvalue _returnvalue_2) (* (`self.Velocidad`) DeltaSeconds))) false false)
          (if (< (`KismetMathLibrary.Vector_Distance` _returnvalue_2 _returnvalue) (`self.Cerca`))
            (set `self.Indice` (+ (`self.Indice`) 1))))))))

(fn `UserConstructionScript`)