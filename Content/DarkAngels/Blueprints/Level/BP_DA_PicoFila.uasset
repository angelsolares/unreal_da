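; BP_DA_PicoFila drives a row of spike actors that rise and sink together and damage the player.
; It collects the actors by tag on BeginPlay, then moves them each Tick along a game-time sine wave with configurable period, phase and travel.
; Hits use no collision: a 2D distance and tip-versus-feet height test applies damage to player 0, throttled by one shared cooldown.
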(event `self.ReceiveBeginPlay`
  (bind _outactors (`GameplayStatics.GetAllActorsWithTag` (`self.EtiquetaFila`)))
  (set `self.PicosFila` _outactors)
  (set `self.Espera` 0.0))

(event `self.ReceiveTick`
  (params (DeltaSeconds :type "Float (single-precision)"))
  (bind _returnvalue (`GameplayStatics.GetPlayerCharacter` 0))
  (set `self.Espera` (- (`self.Espera`) DeltaSeconds))
  (for _array_element (`self.PicosFila`)
    (`self.K2_SetActorLocation` _array_element (`KismetMathLibrary.MakeVector` (.x (`self.K2_GetActorLocation` _array_element)) (.y (`self.K2_GetActorLocation` _array_element)) (+ (- (`self.ZArriba`) (`self.Recorrido`)) (* (`self.Recorrido`) (* 0.5 (+ 1.0 (`KismetMathLibrary.DegSin` (* 360.0 (+ (/ (`KismetSystemLibrary.GetGameTimeInSeconds`) (`self.Periodo`)) (`self.Fase`))))))))) false false)
    (if (and (<= (`self.Espera`) 0.0) (and (< (`KismetMathLibrary.Vector_Distance2D` (`self.K2_GetActorLocation` _returnvalue) (`self.K2_GetActorLocation` _array_element)) (`self.RadioDano`)) (> (- (+ (.z (`self.K2_GetActorLocation` _array_element)) (`self.AlturaPunta`)) (- (.z (`self.K2_GetActorLocation` _returnvalue)) (`self.AlturaCapsula`))) (`self.SobresalirMin`))))
      (`GameplayStatics.ApplyDamage` _returnvalue (`self.Dano`) null self)
      (set `self.Espera` (`self.Recarga`)))))

(fn `UserConstructionScript`)