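; Prologue threshold trigger that stages a one-time scripted takedown of the player by the custodian.
; BeginPlay finds the tagged custodian, sword and light beam actors, hides the sword and disarms the player.
; On player overlap, it locks input, cools the light, snaps the player facing the custodian and plays paired montages.
; Afterwards it reveals the sword, warms the light, restores input and updates the HUD objective; unconnected older copies remain.
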(event `self.ReceiveBeginPlay`
  (bind _outactors (`GameplayStatics.GetAllActorsWithTag` "PrologoCustodio"))
  (for _array_element _outactors
    (set `self.Custodio` _array_element))
  (bind _outactors_2 (`GameplayStatics.GetAllActorsWithTag` "PrologoEspada"))
  (for _array_element_2 _outactors_2
    (set `self.Espada` _array_element_2))
  (bind _outactors_3 (`GameplayStatics.GetAllActorsWithTag` "PrologoHaz"))
  (for _array_element_3 _outactors_3
    (set `self.Haz` _array_element_3))
  (`self.SetActorHiddenInGame` (`self.Espada`) true)
  (`KismetSystemLibrary.Delay` 0.2)
  (bind _asbp_da_player_character (cast `/Game/DarkAngels/Blueprints/Characters/BP_DA_PlayerCharacter` (`GameplayStatics.GetPlayerCharacter` 0)))
  (`/Engine/EditorBlueprintResources/StandardMacros.IsValid` _asbp_da_player_character
    (:`Is Valid`
      (`/Game/DarkAngels/Blueprints/Characters/BP_DA_PlayerCharacter.DesarmarAlEmpezar` _asbp_da_player_character))))

(event `self.ReceiveActorBeginOverlap`
  (params (OtherActor :type "Actor Object Reference"))
  (bind _returnvalue (`GameplayStatics.GetPlayerController` 0))
  (bind _asbp_da_player_character (cast `/Game/DarkAngels/Blueprints/Characters/BP_DA_PlayerCharacter` OtherActor))
  (bind _ascharacter (cast `Character` (`self.Custodio`)))
  (`/Engine/EditorBlueprintResources/StandardMacros.IsValid` _asbp_da_player_character
    (:`Is Valid`
      (`/Engine/EditorBlueprintResources/StandardMacros.IsValid` _ascharacter
        (:`Is Valid`
          (if (`self.Disparado`)
            (set `self.Disparado` true)
            (else
              (set `self.Disparado` true)
              (bind _asbp_da_hud (cast `/Game/DarkAngels/Blueprints/UI/BP_DA_HUD` (`PlayerController.GetHUD` _returnvalue)))
              (bind _ascharacter_2 (cast `Character` _asbp_da_player_character))
              (bind _aslight_component (cast `LightComponent` (`self.GetComponentByClass` (`self.Haz`) "/Script/Engine.LightComponent")))
              (`Controller.SetIgnoreMoveInput` _returnvalue true)
              (`Controller.SetIgnoreLookInput` _returnvalue true)
              (`self.DisableInput` _ascharacter_2 _returnvalue)
              (`/Game/DarkAngels/Blueprints/UI/BP_DA_HUD.SetObjective` _asbp_da_hud "El umbral no te reconoce" 2)
              (`LightComponent.SetLightColor` _aslight_component (make `LinearColor` 0.55 0.72 1.0 1.0) true)
              (`LightComponent.SetIntensity` _aslight_component 3000.0)
              (`KismetSystemLibrary.Delay` 1.2)
              (`self.K2_SetActorLocation` _ascharacter_2 (+ (`self.K2_GetActorLocation` _ascharacter) (* (`self.GetActorForwardVector` _ascharacter) 123.0)) false false)
              (`self.K2_SetActorRotation` _ascharacter_2 (`KismetMathLibrary.MakeRotator` 0.0 0.0 (+ (.yaw (`self.K2_GetActorRotation` _ascharacter)) 180.0)) false)
              (bind _returnvalue_2 (`Character.PlayAnimMontage` _ascharacter "/Game/DarkAngels/Animations/Finishers/Sword_Single/AS_Sword_Takedown_01_Montage.AS_Sword_Takedown_01_Montage" 1.0 "None"))
              (`Character.PlayAnimMontage` _ascharacter_2 "/Game/DarkAngels/Animations/Finishers/Sword_Single/AS_Sword_Takedown_01_React_Montage.AS_Sword_Takedown_01_React_Montage" 1.0 "None")
              (`KismetSystemLibrary.Delay` _returnvalue_2)
              (`self.SetActorHiddenInGame` (`self.Espada`) false)
              (`LightComponent.SetLightColor` _aslight_component (make `LinearColor` 1.0 0.96 0.84 1.0) true)
              (`LightComponent.SetIntensity` _aslight_component 18000.0)
              (`self.EnableInput` _ascharacter_2 _returnvalue)
              (`Controller.SetIgnoreMoveInput` _returnvalue false)
              (`Controller.SetIgnoreLookInput` _returnvalue false)
              (`/Game/DarkAngels/Blueprints/UI/BP_DA_HUD.SetObjective` _asbp_da_hud "Toma la espada del custodio" 3))))))))

(fn `UserConstructionScript`)