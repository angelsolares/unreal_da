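; BP_DA_Paso is an interactable passage that teleports the player to a destination actor, gated by GameState flags.
; It opens if it has no requirement, the requirement is held or it was already opened; otherwise a second requirement allows forcing it.
; Forcing locks input during a montage, VFX and delay, then saves the opened flag.
; Crossing marks a passage flag, plays a door sound and aligns player and camera with the destination.
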(event `/Game/DynamicCombatSystem/DCS/Blueprints/Interfaces/I_IsInteractable.Interact`
  (params (Caller :type "Actor Object Reference"))
  (bind _asbp_da_game_state (cast `/Game/DarkAngels/Blueprints/World/BP_DA_GameState` (`GameplayStatics.GetGameState`)))
  (bind _tiene (`/Game/DarkAngels/Blueprints/World/BP_DA_GameState.Lleva` _asbp_da_game_state (`self.FlagAbierta`)))
  (bind _tiene_2 (`/Game/DarkAngels/Blueprints/World/BP_DA_GameState.Lleva` _asbp_da_game_state (`self.Requisito`)))
  (bind _tiene_3 (`/Game/DarkAngels/Blueprints/World/BP_DA_GameState.Lleva` _asbp_da_game_state (`self.RequisitoForzar`)))
  (bind _returnvalue (or (`KismetStringLibrary.IsEmpty` (`self.Requisito`)) (or (and (not (`KismetStringLibrary.IsEmpty` (`self.FlagAbierta`))) _tiene) _tiene_2)))
  (if (and _returnvalue (not (`KismetStringLibrary.IsEmpty` (`self.FlagPaso`))))
    (`/Game/DarkAngels/Blueprints/World/BP_DA_GameState.MarcarFlag` _asbp_da_game_state (`self.FlagPaso`)))
  (if _returnvalue
    (`self.CruzarPaso`))
  (if (and (not _returnvalue) (and (not (`KismetStringLibrary.IsEmpty` (`self.RequisitoForzar`))) _tiene_3))
    (`Controller.SetIgnoreMoveInput` (`GameplayStatics.GetPlayerController` 0) true)
    (`Controller.SetIgnoreLookInput` (`GameplayStatics.GetPlayerController` 0) true)
    (`Character.PlayAnimMontage` (`GameplayStatics.GetPlayerCharacter` 0) (`self.MontageForzar`) 1.0 "None")
    (`NiagaraFunctionLibrary.SpawnSystemAtLocation` (`self.VfxForzar`) (`SceneComponent.K2_GetComponentLocation` (`self.Zona`)))
    (`KismetSystemLibrary.Delay` (`self.EsperaForzar`))
    (`Controller.SetIgnoreMoveInput` (`GameplayStatics.GetPlayerController` 0) false)
    (`Controller.SetIgnoreLookInput` (`GameplayStatics.GetPlayerController` 0) false)
    (bind _asbp_da_game_state_2 (cast `/Game/DarkAngels/Blueprints/World/BP_DA_GameState` (`GameplayStatics.GetGameState`)))
    (`/Game/DarkAngels/Blueprints/World/BP_DA_GameState.MarcarFlag` _asbp_da_game_state_2 (`self.FlagAbierta`))
    (bind _asbp_da_game_state_3 (cast `/Game/DarkAngels/Blueprints/World/BP_DA_GameState` (`GameplayStatics.GetGameState`)))
    (`/Game/DarkAngels/Blueprints/World/BP_DA_GameState.MarcarFlag` _asbp_da_game_state_3 (`self.FlagPaso`))
    (`self.CruzarPaso`)))

(fn `CruzarPaso`
  (bind _returnvalue (`GameplayStatics.GetPlayerCharacter` 0))
  (bind _destino (`self.Destino`))
  (bind _returnvalue_2 (`self.K2_GetActorLocation` _destino))
  (bind _returnvalue_3 (`KismetMathLibrary.MakeRotator` 0.0 0.0 (.yaw (`self.K2_GetActorRotation` _destino))))
  (`GameplayStatics.PlaySound2D` "/Game/DarkAngels/Audio/SFX/door_open.door_open" 1.0 1.0 0.0 null null)
  (`/Engine/EditorBlueprintResources/StandardMacros.IsValid` _destino
    (:`Is Valid`
      (`self.K2_SetActorLocationAndRotation` _returnvalue (`KismetMathLibrary.MakeVector` (.x _returnvalue_2) (.y _returnvalue_2) (+ (.z _returnvalue_2) (+ (`CapsuleComponent.GetScaledCapsuleHalfHeight` (`Character.CapsuleComponent` _returnvalue)) 10.0))) _returnvalue_3 false true)
      (`Controller.SetControlRotation` (`GameplayStatics.GetPlayerController` 0) _returnvalue_3))))

(fn `GetInteractionMessage`
  (returns (Message :type Name))
  (bind _asbp_da_game_state (cast `/Game/DarkAngels/Blueprints/World/BP_DA_GameState` (`GameplayStatics.GetGameState`)))
  (bind _verbo (`/Game/DarkAngels/Blueprints/World/BP_DA_GameState.VerboPaso` _asbp_da_game_state (`self.Requisito`) (`self.RequisitoForzar`) (`self.FlagAbierta`)))
  (return (`KismetStringLibrary.Conv_StringToName` _verbo)))

(fn `UserConstructionScript`)