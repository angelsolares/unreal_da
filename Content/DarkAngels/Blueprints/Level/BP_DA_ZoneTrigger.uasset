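; Level zone trigger that, when the player enters, updates the HUD objective, shows a zone banner and sets a debug zone index.
; BeginPlay sets up the overlap box and zone label, then starts a looping half-second timer.
; Player overlaps fire the entry on every begin, while the timer's axis-aligned point-in-box check fires it once via HasFired, which overlaps never set.
; FireZoneEntryIfInside is not called within this Blueprint.
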(event `self.ReceiveBeginPlay`
  (`PrimitiveComponent.SetCollisionProfileName` (`self.TriggerBox`) "OverlapAllDynamic" true)
  (set `PrimitiveComponent.bGenerateOverlapEvents` true (`self.TriggerBox`))
  (`TextRenderComponent.K2_SetText` (`self.ZoneLabel`) (`self.ZoneName`))
  (`TextRenderComponent.SetTextRenderColor` (`self.ZoneLabel`) (make `Color` 255 215 100 255))
  (`KismetSystemLibrary.K2_SetTimer` self "CheckPlayerInside" 0.5 true))

(event `self.TriggerBox.OnComponentBeginOverlap`
  (params (OverlappedComponent :type "PrimitiveComponent Object Reference") (OtherActor :type "Actor Object Reference") (OtherComp :type "PrimitiveComponent Object Reference") (OtherBodyIndex :type Integer) (bFromSweep :type Boolean) (SweepResult :type "HitResult Structure (by ref)"))
  (cast `/Game/DarkAngels/Blueprints/Characters/BP_DA_PlayerCharacter_V2` OtherActor)
  (`self.FireZoneEntry`))

(fn `CheckPlayerInside`
  (if (not (`self.HasFired`))
    (if (`KismetMathLibrary.IsPointInBox` (`self.K2_GetActorLocation` (`GameplayStatics.GetPlayerCharacter` 0)) (`self.K2_GetActorLocation`) (`BoxComponent.GetScaledBoxExtent` (`self.TriggerBox`)))
      (set `self.HasFired` true)
      (`self.FireZoneEntry`))))

(fn `FireZoneEntry`
  (bind _asbp_da_hud (cast `/Game/DarkAngels/Blueprints/UI/BP_DA_HUD` (`PlayerController.GetHUD` (`GameplayStatics.GetPlayerController` 0))))
  (`/Game/DarkAngels/Blueprints/UI/BP_DA_HUD.SetObjective` _asbp_da_hud (`self.ObjectiveText`) (`self.ObjectiveIndex`))
  (`/Game/DarkAngels/Blueprints/UI/BP_DA_HUD.ShowZoneBanner` _asbp_da_hud (`self.ZoneName`))
  (set `/Game/DarkAngels/Blueprints/UI/BP_DA_HUD.ZonaActualDebug` (`self.IndicePanel`) _asbp_da_hud))

(fn `FireZoneEntryIfInside`
  (`KismetSystemLibrary.PrintString` "DA_TRIGGER: chequeo inicial de zona")
  (if (`self.IsOverlappingActor` (`GameplayStatics.GetPlayerCharacter` 0) self)
    (`self.FireZoneEntry`)))

(fn `UserConstructionScript`)