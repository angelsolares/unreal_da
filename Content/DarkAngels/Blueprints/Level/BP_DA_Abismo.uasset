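; Abyss fall handler that catches the player dropping below a height threshold and offers a respawn.
; Each Tick it checks player Z; on falling it marks a GameState flag and locks move and look input.
; While fallen it keeps showing a HUD banner and polls the R key directly.
; Pressing R teleports the player to the respawn point, matches its yaw, restores input and clears the banner.
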(event `self.ReceiveTick`
  (params (DeltaSeconds :type "Float (single-precision)"))
  (`self.VigilarAbismo`))

(fn `RenacerAbismo`
  (bind _returnvalue (`GameplayStatics.GetPlayerCharacter` 0))
  (bind _returnvalue_2 (`GameplayStatics.GetPlayerController` 0))
  (bind _puntorespawn (`self.PuntoRespawn`))
  (bind _returnvalue_3 (`KismetMathLibrary.MakeRotator` 0.0 0.0 (.yaw (`self.K2_GetActorRotation` _puntorespawn))))
  (`/Engine/EditorBlueprintResources/StandardMacros.IsValid` _puntorespawn
    (:`Is Valid`
      (`MovementComponent.StopMovementImmediately` (`self.GetComponentByClass` _returnvalue "/Script/Engine.CharacterMovementComponent"))
      (`self.K2_SetActorLocationAndRotation` _returnvalue (`self.K2_GetActorLocation` _puntorespawn) _returnvalue_3 false true)
      (`Controller.SetControlRotation` _returnvalue_2 _returnvalue_3)
      (`Controller.SetIgnoreMoveInput` _returnvalue_2 false)
      (`Controller.SetIgnoreLookInput` _returnvalue_2 false)
      (bind _asbp_da_hud (cast `/Game/DarkAngels/Blueprints/UI/BP_DA_HUD` (`PlayerController.GetHUD` _returnvalue_2)))
      (set `/Game/DarkAngels/Blueprints/UI/BP_DA_HUD.ZoneText` "" _asbp_da_hud)
      (set `self.Caido` false))))

(fn `UserConstructionScript`)

(fn `VigilarAbismo`
  (bind _returnvalue (`GameplayStatics.GetPlayerController` 0))
  (if (and (not (`self.Caido`)) (< (.z (`self.K2_GetActorLocation` (`GameplayStatics.GetPlayerCharacter` 0))) (`self.CotaMortal`)))
    (set `self.Caido` true)
    (bind _asbp_da_game_state (cast `/Game/DarkAngels/Blueprints/World/BP_DA_GameState` (`GameplayStatics.GetGameState`)))
    (`/Game/DarkAngels/Blueprints/World/BP_DA_GameState.MarcarFlag` _asbp_da_game_state (`self.Flag`))
    (`Controller.SetIgnoreMoveInput` _returnvalue true)
    (`Controller.SetIgnoreLookInput` _returnvalue true))
  (if (`self.Caido`)
    (bind _asbp_da_hud (cast `/Game/DarkAngels/Blueprints/UI/BP_DA_HUD` (`PlayerController.GetHUD` _returnvalue)))
    (`/Game/DarkAngels/Blueprints/UI/BP_DA_HUD.ShowZoneBanner` _asbp_da_hud (`KismetTextLibrary.Conv_StringToText` (`self.Texto`))))
  (if (and (`self.Caido`) (`PlayerController.WasInputKeyJustPressed` _returnvalue "R"))
    (`self.RenacerAbismo`)))