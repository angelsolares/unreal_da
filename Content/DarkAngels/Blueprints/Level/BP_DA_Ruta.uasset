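; BP_DA_Ruta is a level route actor that lets the player summon a BP_DA_Fuego as an apparent guide for that route.
; Each tick it polls the G key and, if PermiteGuia allows, spawns the Fuego at the player character's transform.
; It passes itself as the route and its EsPrincipal flag to the Fuego, then marks it ready through Listo.
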(event `self.ReceiveTick`
  (params (DeltaSeconds :type "Float (single-precision)"))
  (if (`PlayerController.WasInputKeyJustPressed` (`GameplayStatics.GetPlayerController` 0) "G")
    (if (`self.PermiteGuia`)
      (bind _asbp_da_ruta (cast `/Game/DarkAngels/Blueprints/Level/BP_DA_Ruta` (`ActorComponent.GetOwner` (`self.DefaultSceneRoot`))))
      (bind _returnvalue (`|SpawnActorFromClass` "/Game/DarkAngels/Blueprints/Level/BP_DA_Fuego.BP_DA_Fuego_C" (`self.GetTransform` (`GameplayStatics.GetPlayerCharacter` 0)) "AlwaysSpawn" "MultiplyWithRoot" null null))
      (bind _asbp_da_fuego (cast `/Game/DarkAngels/Blueprints/Level/BP_DA_Fuego` _returnvalue))
      (set `/Game/DarkAngels/Blueprints/Level/BP_DA_Fuego.Ruta` _asbp_da_ruta _asbp_da_fuego)
      (set `/Game/DarkAngels/Blueprints/Level/BP_DA_Fuego.Principal` (`self.EsPrincipal`) _asbp_da_fuego)
      (set `/Game/DarkAngels/Blueprints/Level/BP_DA_Fuego.Listo` true _asbp_da_fuego))))

(fn `UserConstructionScript`)