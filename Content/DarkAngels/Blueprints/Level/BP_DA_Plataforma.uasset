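; BP_DA_Plataforma drives a moving platform by oscillating a referenced actor (Objetivo) back and forth along the world X axis.
; BeginPlay stores the target's starting X and enables movement only if the reference is valid.
; Each Tick, MoverPlataforma sets the location from a game-time sine wave using amplitude, period and phase offset.
; Movement is unswept and keeps the target's current Y and Z.
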(event `self.ReceiveBeginPlay`
  (`/Engine/EditorBlueprintResources/StandardMacros.IsValid` (`self.Objetivo`)
    (:`Is Valid`
      (set `self.OrigenX` (.x (`self.K2_GetActorLocation` (`self.Objetivo`))))
      (set `self.Listo` true))))

(event `self.ReceiveTick`
  (params (DeltaSeconds :type "Float (single-precision)"))
  (`self.MoverPlataforma`))

(fn `MoverPlataforma`
  (bind _objetivo (`self.Objetivo`))
  (bind _returnvalue (`self.K2_GetActorLocation` _objetivo))
  (if (`self.Listo`)
    (`self.K2_SetActorLocation` _objetivo (`KismetMathLibrary.MakeVector` (+ (`self.OrigenX`) (* (`self.Amplitud`) (`KismetMathLibrary.DegSin` (* 360.0 (+ (/ (`KismetSystemLibrary.GetGameTimeInSeconds`) (`self.Periodo`)) (`self.Desfase`)))))) (.y _returnvalue) (.z _returnvalue)) false false)))

(fn `UserConstructionScript`)