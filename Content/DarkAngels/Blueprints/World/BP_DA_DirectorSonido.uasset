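; BP_DA_DirectorSonido is a sound director Blueprint for Dark Angels that controls the background music and ambience.
; Its PonerFondo function takes a new music and ambience sound, then sets and plays each on its own audio component from the start.
; Each track restarts only when its object name differs from the stored current one, so repeat requests leave playback uninterrupted.
; The event graph and construction script are empty.
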(fn `PonerFondo`
  (params (NuevaMusica :type "SoundBase Object Reference") (NuevoAmbiente :type "SoundBase Object Reference"))
  (if (not (`KismetStringLibrary.EqualEqual_StrStr` (`KismetSystemLibrary.GetObjectName` (`self.MusicaActual`)) (`KismetSystemLibrary.GetObjectName` NuevaMusica)))
    (set `self.MusicaActual` NuevaMusica)
    (`AudioComponent.SetSound` (`self.Musica`) NuevaMusica)
    (`AudioComponent.Play` (`self.Musica`) 0.0))
  (if (not (`KismetStringLibrary.EqualEqual_StrStr` (`KismetSystemLibrary.GetObjectName` (`self.AmbienteActual`)) (`KismetSystemLibrary.GetObjectName` NuevoAmbiente)))
    (set `self.AmbienteActual` NuevoAmbiente)
    (`AudioComponent.SetSound` (`self.Ambiente`) NuevoAmbiente)
    (`AudioComponent.Play` (`self.Ambiente`) 0.0)))

(fn `UserConstructionScript`)