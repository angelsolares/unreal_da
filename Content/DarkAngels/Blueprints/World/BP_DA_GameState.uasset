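; Game state for Dark Angels that records the player's Grace, Corruption and Will marks, narrative flags and transformations.
; AnotarMarca logs each mark, bumps its counter and the narrative step count, and plays choice sounds.
; Conjugar maps exactly three marks to one of ten named outcomes, while VerboPaso derives passage verbs (cross, force, sealed) from flags and mark names.
; ReiniciarEsfera resets counters per sphere but keeps history and flags.
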(event `self.ReceiveBeginPlay`)

(fn `AnotarMarca`
  (params (Fuerza :type Integer) (Nombre :type String))
  (`KismetArrayLibrary.Array_Add` (`self.MarcaFuerza`) Fuerza)
  (`KismetArrayLibrary.Array_Add` (`self.MarcaNombre`) Nombre)
  (`self.MarcarEvento`)
  (if (== Fuerza 1)
    (set `self.Gracia` (+ (`self.Gracia`) 1))
    (`GameplayStatics.PlaySound2D` "/Game/DarkAngels/Audio/SFX/choice_grace.choice_grace" 1.0 1.0 0.0 null null)
    (if (== (`self.Gracia`) 2)
      (`GameplayStatics.PlaySound2D` "/Game/DarkAngels/Audio/SFX/mark_awarded.mark_awarded" 1.0 1.0 0.0 null null))
    (elif (== Fuerza 2)
      (set `self.Corrupcion` (+ (`self.Corrupcion`) 1))
      (`GameplayStatics.PlaySound2D` "/Game/DarkAngels/Audio/SFX/choice_corruption.choice_corruption" 1.0 1.0 0.0 null null)
      (if (== (`self.Corrupcion`) 2)
        (`GameplayStatics.PlaySound2D` "/Game/DarkAngels/Audio/SFX/mark_awarded.mark_awarded" 1.0 1.0 0.0 null null))
      (elif (== Fuerza 3)
        (set `self.Voluntad` (+ (`self.Voluntad`) 1))
        (`GameplayStatics.PlaySound2D` "/Game/DarkAngels/Audio/SFX/choice_will.choice_will" 1.0 1.0 0.0 null null)
        (if (== (`self.Voluntad`) 2)
          (`GameplayStatics.PlaySound2D` "/Game/DarkAngels/Audio/SFX/mark_awarded.mark_awarded" 1.0 1.0 0.0 null null))))))

(fn `BorrarTodo`
  (set `self.Gracia` 0)
  (set `self.Corrupcion` 0)
  (set `self.Voluntad` 0)
  (`KismetArrayLibrary.Array_Clear` (`self.MarcaFuerza`))
  (`KismetArrayLibrary.Array_Clear` (`self.MarcaNombre`))
  (`KismetArrayLibrary.Array_Clear` (`self.Flags`)))

(fn `Conjugar`
  (returns (Texto :type String))
  (return (select `bool` (< (+ (+ (`self.Gracia`) (`self.Corrupcion`)) (`self.Voluntad`)) 3) :`false` (select `bool` (> (+ (+ (`self.Gracia`) (`self.Corrupcion`)) (`self.Voluntad`)) 3) :`false` (select `bool` (and (== (`self.Gracia`) 3) (and (== (`self.Corrupcion`) 0) (== (`self.Voluntad`) 0))) :`false` (select `bool` (and (== (`self.Gracia`) 0) (and (== (`self.Corrupcion`) 3) (== (`self.Voluntad`) 0))) :`false` (select `bool` (and (== (`self.Gracia`) 0) (and (== (`self.Corrupcion`) 0) (== (`self.Voluntad`) 3))) :`false` (select `bool` (and (== (`self.Gracia`) 2) (and (== (`self.Corrupcion`) 1) (== (`self.Voluntad`) 0))) :`false` (select `bool` (and (== (`self.Gracia`) 2) (and (== (`self.Corrupcion`) 0) (== (`self.Voluntad`) 1))) :`false` (select `bool` (and (== (`self.Gracia`) 1) (and (== (`self.Corrupcion`) 2) (== (`self.Voluntad`) 0))) :`false` (select `bool` (and (== (`self.Gracia`) 0) (and (== (`self.Corrupcion`) 2) (== (`self.Voluntad`) 1))) :`false` (select `bool` (and (== (`self.Gracia`) 1) (and (== (`self.Corrupcion`) 0) (== (`self.Voluntad`) 2))) :`false` (select `bool` (and (== (`self.Gracia`) 0) (and (== (`self.Corrupcion`) 1) (== (`self.Voluntad`) 2))) :`false` (select `bool` (and (== (`self.Gracia`) 1) (and (== (`self.Corrupcion`) 1) (== (`self.Voluntad`) 1))) :`false` "Sin resolver" :`true` "10 · Gracia + Corrupción + Voluntad — Convergente") :`true` "9 · Voluntad + Voluntad + Corrupción — Libre Oscuro") :`true` "8 · Voluntad + Voluntad + Gracia — Libre Luminoso") :`true` "7 · Corrupción + Corrupción + Voluntad — Renegado") :`true` "6 · Corrupción + Corrupción + Gracia — Eclipse Oscuro") :`true` "5 · Gracia + Gracia + Voluntad — Heraldo Libre") :`true` "4 · Gracia + Gracia + Corrupción — Eclipse Celestial") :`true` "3 · Voluntad Pura — Desatado de Malkuth") :`true` "2 · Corrupción Pura — Corrupto de Malkuth") :`true` "1 · Gracia Pura — Ascendido de Malkuth") :`true` (`KismetStringLibrary.Concat_StrStr` "Sin conjunción: " (`KismetStringLibrary.Concat_StrStr` (`KismetStringLibrary.Conv_IntToString` (+ (+ (`self.Gracia`) (`self.Corrupcion`)) (`self.Voluntad`))) " marcas, deberían ser 3"))) :`true` (`KismetStringLibrary.Concat_StrStr` "Sin conjunción: faltan marcas (" (`KismetStringLibrary.Concat_StrStr` (`KismetStringLibrary.Conv_IntToString` (+ (+ (`self.Gracia`) (`self.Corrupcion`)) (`self.Voluntad`))) " de 3)")))))

(fn `FuerzaEnPaso`
  (params (Indice :type Integer))
  (returns (Valor :type Integer))
  (bind _marcafuerza (`self.MarcaFuerza`))
  (if (`KismetArrayLibrary.Array_IsValidIndex` _marcafuerza Indice)
    (return (`|GetArrayItem` _marcafuerza Indice))
    (else
      (return 0))))

(fn `GuardarTransformacion`
  (params (Texto :type String))
  (set `self.Transformacion` Texto)
  (`KismetArrayLibrary.Array_Add` (`self.Transformaciones`) Texto))

(fn `Historial`
  (returns (Texto :type String))
  (return (`KismetStringLibrary.JoinStringArray` (`self.MarcaNombre`) ", ")))

(fn `LeerFuerza`
  (params (Fuerza :type Integer))
  (returns (Cuantas :type Integer))
  (return (select `bool` (== Fuerza 1) :`false` (select `bool` (== Fuerza 2) :`false` (select `bool` (== Fuerza 3) :`false` 0 :`true` (`self.Voluntad`)) :`true` (`self.Corrupcion`)) :`true` (`self.Gracia`))))

(fn `LeerPasos`
  (returns (Pasos :type Integer))
  (return (`self.PasosNarrativos`)))

(fn `LeerTransformacion`
  (returns (Texto :type String))
  (return (`self.Transformacion`)))

(fn `Lleva`
  (params (Nombre :type String))
  (returns (Tiene :type Boolean))
  (return (or (`KismetArrayLibrary.Array_Contains` (`self.Flags`) Nombre) (`KismetArrayLibrary.Array_Contains` (`self.MarcaNombre`) Nombre))))

(fn `MarcarEvento`
  (set `self.PasosNarrativos` (+ (`self.PasosNarrativos`) 1)))

(fn `MarcarFlag`
  (params (Nombre :type String))
  (`KismetArrayLibrary.Array_AddUnique` (`self.Flags`) Nombre)
  (`self.MarcarEvento`))

(fn `ReiniciarEsfera`
  (params (NuevaEsfera :type String))
  (set `self.Gracia` 0)
  (set `self.Corrupcion` 0)
  (set `self.Voluntad` 0)
  (set `self.Esfera` NuevaEsfera))

(fn `Resumen`
  (returns (Texto :type String))
  (return (`KismetStringLibrary.Concat_StrStr` (`KismetStringLibrary.Concat_StrStr` (`KismetStringLibrary.Concat_StrStr` "G:" (`KismetStringLibrary.Conv_IntToString` (`self.Gracia`))) (`KismetStringLibrary.Concat_StrStr` "   C:" (`KismetStringLibrary.Conv_IntToString` (`self.Corrupcion`)))) (`KismetStringLibrary.Concat_StrStr` "   V:" (`KismetStringLibrary.Conv_IntToString` (`self.Voluntad`))))))

(fn `TieneFlag`
  (params (Nombre :type String))
  (returns (Tiene :type Boolean))
  (return (`KismetArrayLibrary.Array_Contains` (`self.Flags`) Nombre)))

(fn `TotalMarcas`
  (returns (Cuantas :type Integer))
  (return (`KismetArrayLibrary.Array_Length` (`self.MarcaFuerza`))))

(fn `UserConstructionScript`)

(fn `VerboPaso`
  (params (Requerido :type String) (Forzar :type String) (Abierta :type String))
  (returns (Verbo :type String))
  (bind _returnvalue (or (`KismetStringLibrary.IsEmpty` Requerido) (or (and (not (`KismetStringLibrary.IsEmpty` Abierta)) (or (`KismetArrayLibrary.Array_Contains` (`self.Flags`) Abierta) (`KismetArrayLibrary.Array_Contains` (`self.MarcaNombre`) Abierta))) (or (`KismetArrayLibrary.Array_Contains` (`self.Flags`) Requerido) (`KismetArrayLibrary.Array_Contains` (`self.MarcaNombre`) Requerido)))))
  (return (select `bool` _returnvalue :`false` (select `bool` (and (not _returnvalue) (and (not (`KismetStringLibrary.IsEmpty` Forzar)) (or (`KismetArrayLibrary.Array_Contains` (`self.Flags`) Forzar) (`KismetArrayLibrary.Array_Contains` (`self.MarcaNombre`) Forzar)))) :`false` "Sellado - la llave está en el Mirador" :`true` "Forzar") :`true` "Cruzar")))