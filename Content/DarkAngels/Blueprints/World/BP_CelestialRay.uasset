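; BP_CelestialRay is a world hazard that, while active, periodically calls beam strikes near a player within trigger range.
; On a cadence timer it picks a randomized point ahead of the player, where the Aviso light brightens as a telegraph.
; When the countdown ends, it spawns BP_DA_BeamVisual and damages the player inside the impact radius, unless their BP_DA_Vetas component reports that point as silenced.
; Leaving range or deactivation cancels pending strikes.
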(event `self.ReceiveTick`
  (params (DeltaSeconds :type "Float (single-precision)"))
  (bind _returnvalue (`GameplayStatics.GetPlayerCharacter` 0))
  (bind _returnvalue_2 (`self.K2_GetActorLocation` _returnvalue))
  (if (and (`self.Activo`) (< (`KismetMathLibrary.Vector_Distance` (`self.K2_GetActorLocation`) _returnvalue_2) (`self.TriggerRadius`)))
    (set `self.FireTimer` (- (`self.FireTimer`) DeltaSeconds))
    (if (`self.bPendingStrike`)
      (set `self.StrikeTimer` (- (`self.StrikeTimer`) DeltaSeconds))
      (`LightComponent.SetIntensity` (`self.Aviso`) (+ 6000.0 (* 34000.0 (- 1.0 (/ (`self.StrikeTimer`) 1.5)))))
      (if (<= (`self.StrikeTimer`) 0.0)
        (set `self.bPendingStrike` false)
        (`LightComponent.SetIntensity` (`self.Aviso`) 0.0)
        (`|SpawnActorFromClass` "/Game/DarkAngels/Blueprints/World/BP_DA_BeamVisual.BP_DA_BeamVisual_C" (`KismetMathLibrary.MakeTransform` (`self.PuntoImpacto`)) "AlwaysSpawn" "MultiplyWithRoot" self null)
        (bind _asbp_da_vetas (cast `/Game/DarkAngels/Blueprints/Combat/BP_DA_Vetas` (`self.GetComponentByClass` _returnvalue "/Game/DarkAngels/Blueprints/Combat/BP_DA_Vetas.BP_DA_Vetas_C")))
        (`/Engine/EditorBlueprintResources/StandardMacros.IsValid` _asbp_da_vetas
          (:`Is Valid`
            (bind _valor (`/Game/DarkAngels/Blueprints/Combat/BP_DA_Vetas.EnSilencio` _asbp_da_vetas (`self.PuntoImpacto`)))
            (if (and (not _valor) (< (`KismetMathLibrary.Vector_Distance` (`self.PuntoImpacto`) _returnvalue_2) (`self.RadioImpacto`)))
              (`GameplayStatics.ApplyDamage` _returnvalue 25.0 null self)))
          (:`Is Not Valid`
            (if (< (`KismetMathLibrary.Vector_Distance` (`self.PuntoImpacto`) _returnvalue_2) (`self.RadioImpacto`))
              (`GameplayStatics.ApplyDamage` _returnvalue 25.0 null self)))))
      (elif (<= (`self.FireTimer`) 0.0)
        (set `self.bPendingStrike` true)
        (set `self.StrikeTimer` 1.5)
        (set `self.PuntoImpacto` (+ (+ _returnvalue_2 (* (`self.GetActorForwardVector` _returnvalue) (`KismetMathLibrary.RandomFloatInRange` 250.0 (`self.AlcanceDelante`)))) (* (`self.GetActorRightVector` _returnvalue) (`KismetMathLibrary.RandomFloatInRange` -400.0 400.0))))
        (`SceneComponent.K2_SetWorldLocation` (`self.Aviso`) (`self.PuntoImpacto`) false false)
        (`LightComponent.SetLightColor` (`self.Aviso`) (make `LinearColor` 1.0 0.72 0.25 1.0) true)
        (set `self.FireTimer` (`self.Cadencia`))))
    (else
      (set `self.FireTimer` (`self.Cadencia`))
      (set `self.bPendingStrike` false)
      (`LightComponent.SetIntensity` (`self.Aviso`) 0.0))))

(fn `UserConstructionScript`)