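; BP_DA_CierreEsfera is a world trigger that closes out a sphere (esfera) once the player character overlaps it.
; It checks a configurable flag on BP_DA_GameState so it fires only once.
; It then gets the Conjugar result, saves it as a transformation, sets the flag and restarts the sphere with NuevaEsfera.
; After a configurable delay, the HUD shows that result as a zone banner.
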(event `self.ReceiveActorBeginOverlap`
  (params (OtherActor :type "Actor Object Reference"))
  (if (== OtherActor (`GameplayStatics.GetPlayerCharacter` 0))
    (bind _asbp_da_game_state (cast `/Game/DarkAngels/Blueprints/World/BP_DA_GameState` (`GameplayStatics.GetGameState`)))
    (bind _tiene (`/Game/DarkAngels/Blueprints/World/BP_DA_GameState.TieneFlag` _asbp_da_game_state (`self.Flag`)))
    (if (not _tiene)
      (bind _texto (`/Game/DarkAngels/Blueprints/World/BP_DA_GameState.Conjugar` _asbp_da_game_state))
      (`/Game/DarkAngels/Blueprints/World/BP_DA_GameState.GuardarTransformacion` _asbp_da_game_state _texto)
      (`/Game/DarkAngels/Blueprints/World/BP_DA_GameState.MarcarFlag` _asbp_da_game_state (`self.Flag`))
      (`/Game/DarkAngels/Blueprints/World/BP_DA_GameState.ReiniciarEsfera` _asbp_da_game_state (`self.NuevaEsfera`))
      (`KismetSystemLibrary.Delay` (`self.Espera`))
      (bind _asbp_da_hud (cast `/Game/DarkAngels/Blueprints/UI/BP_DA_HUD` (`PlayerController.GetHUD` (`GameplayStatics.GetPlayerController` 0))))
      (`/Game/DarkAngels/Blueprints/UI/BP_DA_HUD.ShowZoneBanner` _asbp_da_hud (`KismetTextLibrary.Conv_StringToText` _texto)))))

(fn `UserConstructionScript`)