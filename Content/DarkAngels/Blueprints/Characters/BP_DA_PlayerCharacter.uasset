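; Dark Angels player character, extending a parent combat character with tech rolls, backstabs and a throwable temporary weapon.
; BeginPlay adds an extra input mapping; roll input can trigger a one-use tech roll that interrupts status and montage.
; Backstab finds a close target, requires it to be alive but damaged, applies a status and spends stamina.
; Throwing spawns a spear along control rotation, removes the temporary weapon and re-equips the base sword if found.
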(event `self.ReceiveBeginPlay`
  (`EnhancedInputSubsystemInterface.AddMappingContext` (pcsubsystem `EnhancedInputLocalPlayerSubsystem` (`GameplayStatics.GetPlayerController` 0)) "/Game/DarkAngels/Input/IMC_DA_Extra.IMC_DA_Extra" 1 (struct))
  (`parent.ReceiveBeginPlay`)
  (set `/Game/DynamicCombatSystem/DCS/Blueprints/Components/BP_DynamicTargetingComponent.CanCycleDirectionalTargets` true (`self.DynamicTargeting`))
  (set `/Game/DynamicCombatSystem/DCS/Blueprints/Components/CollisionHandler/BP_CollisionHandlerComponent.Debug` false (`self.MeleeCollisionHandler`)))

(event `self.ReceiveTick`
  (params (DeltaSeconds :type "Float (single-precision)"))
  (`parent.ReceiveTick` DeltaSeconds))

(event `EnhancedInput|/Game/DynamicCombatSystem/DCS/Inputs/IA_Roll`
  (params (ActionValue :type Boolean) (ElapsedSeconds :type "Float (double-precision)") (TriggeredSeconds :type "Float (double-precision)") (InputAction :type "InputAction Object Reference" :default "/Game/DynamicCombatSystem/DCS/Inputs/IA_Roll.IA_Roll"))
  (:`Started`
    (`self.TryTechRoll`)))

(event `EnhancedInput|/Game/DarkAngels/Input/IA_DA_Arrojar`
  (params (ActionValue :type Boolean) (ElapsedSeconds :type "Float (double-precision)") (TriggeredSeconds :type "Float (double-precision)") (InputAction :type "InputAction Object Reference" :default "/Game/DarkAngels/Input/IA_DA_Arrojar.IA_DA_Arrojar"))
  (:`Started`
    (`self.ArrojarArmaTemporal`)))

(fn `ArrojarArmaTemporal`
  (bind _armatemporal (`self.ArmaTemporal`))
  (bind _inventory (`self.Inventory`))
  (bind _returnvalue (`self.GetControlRotation` self))
  (`/Engine/EditorBlueprintResources/StandardMacros.IsValid` _armatemporal
    (:`Is Valid`
      (`|SpawnActorFromClass` "/Game/DarkAngels/Weapons/Projectiles/BP_DA_LanzaArrojada.BP_DA_LanzaArrojada_C" (`KismetMathLibrary.MakeTransform` (+ (`self.K2_GetActorLocation` self) (+ (* (`KismetMathLibrary.Conv_RotatorToVector` _returnvalue) 110.0) (`KismetMathLibrary.MakeVector` 0.0 0.0 60.0))) _returnvalue) "AlwaysSpawn" "MultiplyWithRoot" self 60.0 4200.0 6000.0 false null)
      (`/Game/DynamicCombatSystem/DCS/Blueprints/Components/Inventory/BP_InventoryComponent.RemoveItem` _inventory _armatemporal false 1)
      (bind (_itemfound _index) (`/Game/DynamicCombatSystem/DCS/Blueprints/Components/Inventory/BP_InventoryComponent.FindItem` _inventory (`self.EspadaBase`)))
      (if _itemfound
        (`/Game/DynamicCombatSystem/DCS/Blueprints/Components/Inventory/BP_EquipmentComponent.UpdateItemInSlot` (`self.Equipment`) "NewEnumerator18" 0 0 (`/Game/DynamicCombatSystem/DCS/Blueprints/Components/Inventory/BP_InventoryComponent.GetItemAtIndex` _inventory _index) "NewEnumerator1"))
      (set `self.ArmaTemporal` null))))

(fn `CanBeAttacked`
  (returns (Result :type Boolean))
  (bind _statemanager (`self.StateManager`))
  (if (`/Game/DynamicCombatSystem/DCS/Blueprints/Components/StateManager/BP_StateManagerComponent.IsInState` _statemanager "NewEnumerator6")
    (return false)
    (else
      (return (not (or (`/Game/DynamicCombatSystem/DCS/Blueprints/Components/StateManager/BP_StateManagerComponent.HasActivity` _statemanager (struct :`GameplayTags` (struct :`(TagName` "Activity.IsImmortal"))) "NewEnumerator0") (`/Game/DynamicCombatSystem/DCS/Blueprints/Components/StateManager/BP_StateManagerComponent.IsInState` _statemanager "NewEnumerator5")))))))

(fn `SustituirArmaTemporal`
  (params (NuevaArma :type "/Game/DynamicCombatSystem/DCS/Blueprints/Items/ObjectItems/BP_DA_Item_Base Object Reference"))
  (bind _armatemporal (`self.ArmaTemporal`))
  (`/Engine/EditorBlueprintResources/StandardMacros.IsValid` _armatemporal
    (:`Is Valid`
      (bind _asbp_inventory_component (cast `/Game/DynamicCombatSystem/DCS/Blueprints/Components/Inventory/BP_InventoryComponent` (`self.GetComponentByClass` self "/Game/DynamicCombatSystem/DCS/Blueprints/Components/Inventory/BP_InventoryComponent.BP_InventoryComponent_C"))
        (:`then`
          (`/Game/DynamicCombatSystem/DCS/Blueprints/Components/Inventory/BP_InventoryComponent.RemoveItem` _asbp_inventory_component _armatemporal false 1)
          (set `self.ArmaTemporal` NuevaArma))
        (:`CastFailed`
          (set `self.ArmaTemporal` NuevaArma))))
    (:`Is Not Valid`
      (set `self.ArmaTemporal` NuevaArma))))

(fn `TryBackstab`
  (returns (Result :type Boolean))
  (bind _statsmanager (`self.StatsManager`))
  (if (and (`self.CanMeleeAttack`) (not (`NavMovementComponent.IsFalling` (`self.CharacterMovement`))))
    (bind (_foundtarget _targetactor) (`/Game/DynamicCombatSystem/DCS/Blueprints/Components/BP_DynamicTargetingComponent.FindTarget` (`self.DynamicTargeting`) 150.0 (select `bool` (`self.HasMovementInput`) :`false` (`self.K2_GetActorRotation`) :`true` (`KismetMathLibrary.Conv_VectorToRotator` (`self.GetLastMovementInputVector`))) 0.5))
    (if _foundtarget
      (if (and (> (`/Game/DynamicCombatSystem/DCS/Blueprints/Components/StatsManager/BP_StatsManagerComponent.GetStatValue` (`self.GetComponentByClass` _targetactor "/Game/DynamicCombatSystem/DCS/Blueprints/Components/StatsManager/BP_StatsManagerComponent.BP_StatsManagerComponent_C") (struct :`TagName` "Stat.Health.Current") true) 0.0) (<= (/ (`/Game/DynamicCombatSystem/DCS/Blueprints/Components/StatsManager/BP_StatsManagerComponent.GetStatValue` (`self.GetComponentByClass` _targetactor "/Game/DynamicCombatSystem/DCS/Blueprints/Components/StatsManager/BP_StatsManagerComponent.BP_StatsManagerComponent_C") (struct :`TagName` "Stat.Health.Current") true) (`/Game/DynamicCombatSystem/DCS/Blueprints/Components/StatsManager/BP_StatsManagerComponent.GetStatValue` (`self.GetComponentByClass` _targetactor "/Game/DynamicCombatSystem/DCS/Blueprints/Components/StatsManager/BP_StatsManagerComponent.BP_StatsManagerComponent_C") (struct :`TagName` "Stat.Health.Max") true)) 0.95))
        (bind _applied (`/Game/DynamicCombatSystem/DCS/Blueprints/BP_DCSLibrary.ApplyStatus` _targetactor self "NewEnumerator5"))
        (if _applied
          (`/Game/DynamicCombatSystem/DCS/Blueprints/Components/StatsManager/BP_StatsManagerComponent.ModifyStat` _statsmanager (struct :`TagName` "Stat.Stamina.Current") -40.0)
          (`/Game/DynamicCombatSystem/DCS/Blueprints/Components/StatsManager/BP_StatsManagerComponent.InterruptRegeneration` _statsmanager (struct :`TagName` "Stat.Stamina.Current"))
          (return true)
          (else
            _)))))
  (return false))

(fn `TryTechRoll`
  (if (`self.CanTechRoll`)
    (set `self.CanTechRoll` false)
    (`/Game/DynamicCombatSystem/DCS/Blueprints/Components/StatusEffects/BP_StatusEffectsComponent.InterruptStatus` (`self.StatusEffects`) "NewEnumerator2")
    (`self.StopAnimMontage` null)
    (`self.Roll`)))

(fn `UserConstructionScript`
  (`parent.UserConstructionScript`))