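; Player character for Dark Angels, with a Dark Strike attack, toggleable wing glide, altar checkpoints and Farsa/Corruptio meters.
; Tick edge-detects polled input: Dark Strike spends Corruptio to lunge and damage nearby "Angel"-tagged actors on cooldown, while airborne jump toggles reduced gravity.
; Damage drains StatsManager health; death shrinks max Farsa, refills health and returns to the altar checkpoint.
; Every AddFarsa call here passes zero, so it only clamps.
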(event `self.ReceiveBeginPlay`
  (`parent.ReceiveBeginPlay`))

(event `self.ReceiveActorBeginOverlap`
  (params (OtherActor :type "Actor Object Reference"))
  (`parent.ReceiveActorBeginOverlap` OtherActor))

(event `self.ReceiveTick`
  (params (DeltaSeconds :type "Float (single-precision)"))
  (bind _returnvalue (`|GetInputActionValue`))
  (bind _returnvalue_2 (`|GetInputActionValue`))
  (bind _charactermovement (`self.CharacterMovement`))
  (bind _returnvalue_3 (`NavMovementInterface.IsFalling` _charactermovement))
  (set `self.DarkStrikeCooldown` (- (`self.DarkStrikeCooldown`) DeltaSeconds))
  (if (and _returnvalue (not (`self.bThrustPrev`)))
    (if (and (>= (`self.Corruptio`) 30.0) (<= (`self.DarkStrikeCooldown`) 0.0))
      (`self.AddFarsa` 0.0)
      (set `self.Corruptio` (- (`self.Corruptio`) 30.0))
      (set `self.DarkStrikeCooldown` 8.0)
      (`self.LaunchCharacter` (* (`self.GetActorForwardVector`) 800.0) true)
      (bind _outactors (`GameplayStatics.GetAllActorsWithTag` "Angel"))
      (for _array_element _outactors
        (if (< (`KismetMathLibrary.Vector_Distance` (`self.K2_GetActorLocation`) (`self.K2_GetActorLocation` _array_element)) 500.0)
          (`GameplayStatics.ApplyDamage` _array_element 60.0 null self)))
      (`KismetSystemLibrary.PrintString` "DARK STRIKE")
      (else
        (`KismetSystemLibrary.PrintString` "Dark Strike not ready"))))
  (set `self.bThrustPrev` _returnvalue)
  (if (and _returnvalue_2 (and (and (not (`self.bJumpPrev`)) (`self.bWingsUnlocked`)) _returnvalue_3))
    (if (`self.bGliding`)
      (set `self.bGliding` false)
      (set `CharacterMovementComponent.GravityScale` 1.0 _charactermovement)
      (else
        (set `self.bGliding` true)
        (set `CharacterMovementComponent.GravityScale` (`self.GlideGravityScale`) _charactermovement))))
  (set `self.bJumpPrev` _returnvalue_2)
  (if (and (`self.bGliding`) (not _returnvalue_3))
    (set `self.bGliding` false)
    (set `CharacterMovementComponent.GravityScale` 1.0 _charactermovement)))

(event `self.ReceiveAnyDamage`
  (params (Damage :type "Float (single-precision)") (DamageType :type "DamageType Object Reference") (InstigatedBy :type "Controller Object Reference") (DamageCauser :type "Actor Object Reference"))
  (bind _statsmanager (`self.StatsManager`))
  (bind _returnvalue (- (`/Game/DynamicCombatSystem/DCS/Blueprints/Components/StatsManager/BP_StatsManagerComponent.GetStatValue` _statsmanager (struct :`TagName` "Stat.Health.Current") true) Damage))
  (`/Game/DynamicCombatSystem/DCS/Blueprints/Components/StatsManager/BP_StatsManagerComponent.SetStat` _statsmanager (struct :`TagName` "Stat.Health.Current") _returnvalue)
  (if (`self.ActorHasTag` DamageCauser "Angel")
    (`self.AddFarsa` 0.0))
  (if (<= _returnvalue 0.0)
    (`KismetSystemLibrary.PrintString` "DEATH - Mancha de Sombra")
    (set `self.MaxFarsa` (select `bool` (< (- (`self.MaxFarsa`) 10.0) 50.0) :`false` (- (`self.MaxFarsa`) 10.0) :`true` 50.0))
    (if (> (`self.Farsa`) (`self.MaxFarsa`))
      (set `self.Farsa` (`self.MaxFarsa`)))
    (`/Game/DynamicCombatSystem/DCS/Blueprints/Components/StatsManager/BP_StatsManagerComponent.SetStat` _statsmanager (struct :`TagName` "Stat.Health.Current") 100.0)
    (if (`self.bHasCheckpoint`)
      (`self.K2_SetActorLocation` self (`self.CheckpointLocation`) false false))))

(fn `AddCorruptio`
  (params (Delta :type "Float (double-precision)"))
  (bind _returnvalue (+ (`self.Corruptio`) Delta))
  (set `self.Corruptio` (select `bool` (< _returnvalue 0.0) :`false` (select `bool` (> _returnvalue 100.0) :`false` _returnvalue :`true` 100.0) :`true` 0.0)))

(fn `AddFarsa`
  (params (Delta :type "Float (double-precision)"))
  (bind _returnvalue (+ (`self.Farsa`) Delta))
  (set `self.Farsa` (select `bool` (< _returnvalue 0.0) :`false` (select `bool` (> _returnvalue (`self.MaxFarsa`)) :`false` _returnvalue :`true` (`self.MaxFarsa`)) :`true` 0.0)))

(fn `GetCorruptioValue`
  (returns (Value :type "Float (double-precision)"))
  (return (`self.Corruptio`)))

(fn `GetFarsaValue`
  (returns (ReturnValue :type "Float (double-precision)"))
  (return (`self.Farsa`)))

(fn `RestAtAltar`
  (bind _returnvalue (+ (`self.AltarUseCount`) 1))
  (`/Game/DynamicCombatSystem/DCS/Blueprints/Components/StatsManager/BP_StatsManagerComponent.SetStat` (`self.StatsManager`) (struct :`TagName` "Stat.Health.Current") 100.0)
  (set `self.TearsOfRepentance` 3)
  (set `self.bHasCheckpoint` true)
  (set `self.CheckpointLocation` (`self.K2_GetActorLocation`))
  (set `self.AltarUseCount` _returnvalue)
  (`self.AddFarsa` 0.0)
  (if (> _returnvalue 1)
    (`self.AddFarsa` 0.0))
  (`KismetSystemLibrary.PrintString` "Altar: HP restored, checkpoint set"))

(fn `RestoreHealth`
  (`/Game/DynamicCombatSystem/DCS/Blueprints/Components/StatsManager/BP_StatsManagerComponent.SetStat` (`self.StatsManager`) (struct :`TagName` "Stat.Health.Current") 100.0))

(fn `UserConstructionScript`
  (`parent.UserConstructionScript`))