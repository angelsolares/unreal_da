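; Giant boss enemy character for Dark Angels, with melee attacks, AI health and stamina bars, and lock-on targeting.
; Melee socket traces damage enemies, then play a knockdown montage and apply a Knockdown status effect.
; TakeDamage feeds StatsManager alongside its own health counter; at zero it hides the bars, stops AI, movement and montages, ragdolls and dissolves, then destroys itself when the dissolve finishes.
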(event `self.ReceiveBeginPlay`
  (bind _meleecollisionhandler (`self.MeleeCollisionHandler`))
  (set `self.MaxHealth` 200.0)
  (set `self.CurrentHealth` 200.0)
  (set `self.IsDead` false)
  (set `self.AttackDamage` 25.0)
  (`/Game/DynamicCombatSystem/DCS/Blueprints/Components/CollisionHandler/BP_CollisionHandlerComponent.SetCollisionMesh` _meleecollisionhandler (make `/Game/DynamicCombatSystem/DCS/Blueprints/Components/CollisionHandler/F_CollisionComponent` (`self.Mesh`) (`self.AttackSockets`)))
  (set `/Game/DynamicCombatSystem/DCS/Blueprints/Components/CollisionHandler/BP_CollisionHandlerComponent.Debug` false _meleecollisionhandler)
  (`KismetSystemLibrary.Delay` 0.2)
  (bind _aswb_aistat_bars (cast `/Game/DynamicCombatSystem/DCS/Widgets/Stats/WB_AIStatBars` (`WidgetComponent.GetUserWidgetObject` (`self.StatBarsWidget`))))
  (`/Game/DynamicCombatSystem/DCS/Widgets/Stats/WB_StatBar.Initialize` (`/Game/DynamicCombatSystem/DCS/Widgets/Stats/WB_AIStatBars.Health` _aswb_aistat_bars) (`self.StatsManager`) true)
  (`/Game/DynamicCombatSystem/DCS/Widgets/Stats/WB_StatBar.Initialize` (`/Game/DynamicCombatSystem/DCS/Widgets/Stats/WB_AIStatBars.Stamina` _aswb_aistat_bars) (`self.StatsManager`) true))

(event `self.MeleeCollisionHandler.OnHit`
  (params (HitResult :type "HitResult Structure"))
  (bind (_bblockinghit _binitialoverlap _time _distance _location _impactpoint _normal _impactnormal _physmat _hitactor) (`GameplayStatics.BreakHitResult` HitResult))
  (if (`/Game/DynamicCombatSystem/DCS/Blueprints/BP_DCSLibrary.IsEnemy` self _hitactor)
    (bind _asbp_state_manager_component (cast `/Game/DynamicCombatSystem/DCS/Blueprints/Components/StateManager/BP_StateManagerComponent` (`self.GetComponentByClass` _hitactor "/Game/DynamicCombatSystem/DCS/Blueprints/Components/StateManager/BP_StateManagerComponent.BP_StateManagerComponent_C"))
      (:`then`
        (`/Game/DynamicCombatSystem/DCS/Blueprints/Components/StateManager/BP_StateManagerComponent.AddActivityForDuration` _asbp_state_manager_component (struct :`TagName` "Activity.HasPlayedGetHitEffects") false 0.5 false)
        (bind _result (message `/Game/DynamicCombatSystem/DCS/Blueprints/Interfaces/I_CanBeAttacked.TakeDamage` _hitactor (make `/Game/DynamicCombatSystem/DCS/Structs/F_HitData` (`self.AttackDamage`) self (`KismetMathLibrary.GetDirectionUnitVector` (`self.K2_GetActorLocation`) (`self.K2_GetActorLocation` _hitactor)) HitResult (struct :`GameplayTags` (struct :`(TagName` "HitData.CanBeBlocked"))))))
        (if _result
          (bind _ascharacter (cast `Character` _hitactor))
          (`self.StopAnimMontage` _ascharacter null)
          (`self.PlayAnimMontage` _ascharacter "/Game/DarkAngels/Animations/Player/AM_DA_Knockdown.AM_DA_Knockdown" 2.5 "None")
          (`/Game/DynamicCombatSystem/DCS/Blueprints/Components/StatusEffects/BP_StatusEffectsComponent.ApplyStatusByParams` (`self.GetComponentByClass` _hitactor "/Game/DynamicCombatSystem/DCS/Blueprints/Components/StatusEffects/BP_StatusEffectsComponent.BP_StatusEffectsComponent_C") self (make `/Game/DynamicCombatSystem/DCS/Blueprints/Components/StatusEffects/F_StatusEffectParams` 2.39 "/Game/DarkAngels/Blueprints/Combat/BP_DA_StatusEffectLogic_Knockdown.BP_DA_StatusEffectLogic_Knockdown_C" "NewEnumerator2" null 0.0 null))))
      (:`CastFailed`
        (bind _result_2 (message `/Game/DynamicCombatSystem/DCS/Blueprints/Interfaces/I_CanBeAttacked.TakeDamage` _hitactor (make `/Game/DynamicCombatSystem/DCS/Structs/F_HitData` (`self.AttackDamage`) self (`KismetMathLibrary.GetDirectionUnitVector` (`self.K2_GetActorLocation`) (`self.K2_GetActorLocation` _hitactor)) HitResult (struct :`GameplayTags` (struct :`(TagName` "HitData.CanBeBlocked"))))))
        (if _result_2
          (bind _ascharacter_2 (cast `Character` _hitactor))
          (`self.StopAnimMontage` _ascharacter_2 null)
          (`self.PlayAnimMontage` _ascharacter_2 "/Game/DarkAngels/Animations/Player/AM_DA_Knockdown.AM_DA_Knockdown" 2.5 "None")
          (`/Game/DynamicCombatSystem/DCS/Blueprints/Components/StatusEffects/BP_StatusEffectsComponent.ApplyStatusByParams` (`self.GetComponentByClass` _hitactor "/Game/DynamicCombatSystem/DCS/Blueprints/Components/StatusEffects/BP_StatusEffectsComponent.BP_StatusEffectsComponent_C") self (make `/Game/DynamicCombatSystem/DCS/Blueprints/Components/StatusEffects/F_StatusEffectParams` 2.39 "/Game/DarkAngels/Blueprints/Combat/BP_DA_StatusEffectLogic_Knockdown.BP_DA_StatusEffectLogic_Knockdown_C" "NewEnumerator2" null 0.0 null)))))))

(event `self.DissolveEffect.OnDissolveFinished`
  (params (Component :type "PrimitiveComponent Object Reference") (Reversed :type Boolean))
  (`self.K2_DestroyActor` self))

(fn `IsAlive`
  (returns (Result :type Boolean))
  (return (not (`self.IsDead`))))

(fn `IsTargetable`
  (returns (`return value` :type Boolean))
  (return (not (`self.IsDead`))))

(fn `OnDeselected`
  (returns (DummyValue :type Boolean))
  (`SceneComponent.SetHiddenInGame` (`self.TargetWidget`) true true)
  (return false))

(fn `OnSelected`
  (returns (DummyValue :type Boolean))
  (`SceneComponent.SetHiddenInGame` (`self.TargetWidget`) false true)
  (return false))

(fn `TakeDamage`
  (params (HitData :type "/Game/DynamicCombatSystem/DCS/Structs/F_HitData Structure (by ref)"))
  (returns (Result :type Boolean) (ResponseType :type "/Game/DynamicCombatSystem/DCS/Blueprints/Components/Combat/E_AttackResponse Enum"))
  (bind _damage (break `/Game/DynamicCombatSystem/DCS/Structs/F_HitData` HitData))
  (if (or (`self.IsDead`) (<= _damage 0.0))
    (return false "NewEnumerator1")
    (else
      (`/Game/DynamicCombatSystem/DCS/Blueprints/Components/StatsManager/BP_StatsManagerComponent.TakeDamage` (`self.StatsManager`) _damage false)
      (set `self.CurrentHealth` (- (`self.CurrentHealth`) _damage))
      (if (<= (`self.CurrentHealth`) 0.0)
        (set `self.CurrentHealth` 0.0)
        (set `self.IsDead` true)
        (`SceneComponent.SetVisibility` (`self.StatBarsWidget`) false true)
        (`self.StopAnimMontage` self null)
        (`BrainComponent.StopLogic` (`AIController.BrainComponent` (`AIBlueprintHelperLibrary.GetAIController` self)) "Dead")
        (`Controller.StopMovement` (`AIBlueprintHelperLibrary.GetAIController` self))
        (`MovementComponent.StopMovementImmediately` (`self.CharacterMovement`))
        (`CharacterMovementComponent.DisableMovement` (`self.CharacterMovement`))
        (`PrimitiveComponent.SetCollisionEnabled` (`self.CapsuleComponent`) "NoCollision")
        (`PrimitiveComponent.SetCollisionObjectType` (`self.Mesh`) "ECC_PhysicsBody")
        (`PrimitiveComponent.SetCollisionEnabled` (`self.Mesh`) "QueryAndPhysics")
        (`PrimitiveComponent.SetSimulatePhysics` (`self.Mesh`) true)
        (`/Game/DynamicCombatSystem/DCS/Blueprints/Components/Dissolve/BP_DissolveComponent.StartDissolve` (`self.DissolveEffect`) (`self.Mesh`) false))
      (return true "NewEnumerator0"))))

(fn `UserConstructionScript`
  (`parent.UserConstructionScript`))