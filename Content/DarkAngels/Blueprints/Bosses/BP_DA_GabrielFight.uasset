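; Directs the Gabriel boss fight, a mirror labyrinth with questions that damage the player on wrong answers.
; A looping timer polls distance and health to advance three phases: question, shrinking labyrinth with nearby angel descents, then shattered mirrors.
; In the last phase, health drops while the player stands on Gabriel's offset shadow deal bonus damage.
; Gabriel and mirrors are found by tag, or by class and ring radius while Gabriel is invalid.
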(event `self.ReceiveBeginPlay`
  (bind _outactors (`GameplayStatics.GetAllActorsWithTag` "GabrielJefe"))
  (for _array_element _outactors
    (set `self.Gabriel` _array_element))
  (bind _outactors_2 (`GameplayStatics.GetAllActorsWithTag` "EspejoGabriel"))
  (set `self.Espejos` _outactors_2)
  (`KismetSystemLibrary.K2_SetTimer` self "Vigilar" 0.25 true))

(fn `EncogerLaberinto`
  (for _array_element (`self.Espejos`)
    (if (< (`KismetMathLibrary.Vector_Distance` (`self.K2_GetActorLocation` _array_element) (`self.K2_GetActorLocation` (`self.Gabriel`))) (`self.RadioCerca`))
      (`self.SetActorHiddenInGame` _array_element true)
      (`self.SetActorEnableCollision` _array_element false)))
  (bind _outactors (`GameplayStatics.GetAllActorsOfClass` "/Game/DarkAngels/Blueprints/Combat/BP_DA_DescensoAngeles.BP_DA_DescensoAngeles_C"))
  (for _array_element_2 _outactors
    (if (< (`KismetMathLibrary.Vector_Distance` (`self.K2_GetActorLocation` _array_element_2) (`self.K2_GetActorLocation`)) 3000.0)
      (bind _asbp_da_descenso_angeles (cast `/Game/DarkAngels/Blueprints/Combat/BP_DA_DescensoAngeles` _array_element_2))
      (`/Game/DarkAngels/Blueprints/Combat/BP_DA_DescensoAngeles.Arrancar` _asbp_da_descenso_angeles))))

(fn `RecogerEspejos`
  (bind _outactors (`GameplayStatics.GetAllActorsOfClass` "/Game/DarkAngels/Blueprints/Bosses/BP_DA_GiantBoss.BP_DA_GiantBoss_C"))
  (for _array_element _outactors
    (set `self.Gabriel` _array_element))
  (`KismetArrayLibrary.Array_Clear` (`self.Espejos`))
  (bind _outactors_2 (`GameplayStatics.GetAllActorsOfClass` "/Script/Engine.StaticMeshActor"))
  (for _array_element_2 _outactors_2
    (if (and (> (`KismetMathLibrary.Vector_Distance2D` (`self.K2_GetActorLocation` _array_element_2) (`self.K2_GetActorLocation`)) (`self.AnilloMin`)) (< (`KismetMathLibrary.Vector_Distance2D` (`self.K2_GetActorLocation` _array_element_2) (`self.K2_GetActorLocation`)) (`self.AnilloMax`)))
      (`KismetArrayLibrary.Array_Add` (`self.Espejos`) _array_element_2))))

(fn `Responder`
  (params (Eleccion :type Integer))
  (if (`self.PreguntaActiva`)
    (set `self.PreguntaActiva` false)
    (if (== Eleccion (`self.RespuestaCorrecta`))
      (`KismetSystemLibrary.PrintString` "GABRIEL: la respuesta le vale - los espejos callan")
      (else
        (`KismetSystemLibrary.PrintString` "GABRIEL: respuesta equivocada - los espejos disparan")
        (`GameplayStatics.ApplyDamage` (`GameplayStatics.GetPlayerCharacter` 0) 25.0 null self)))))

(fn `RomperEspejos`
  (for _array_element (`self.Espejos`)
    (`self.SetActorHiddenInGame` _array_element true)
    (`self.SetActorEnableCollision` _array_element false)))

(fn `UserConstructionScript`)

(fn `Vigilar`
  (bind _returnvalue (`GameplayStatics.GetPlayerCharacter` 0))
  (`/Engine/EditorBlueprintResources/StandardMacros.IsValid` (`self.Gabriel`)
    (:`Is Valid`
      (bind _asbp_stats_manager_component (cast `/Game/DynamicCombatSystem/DCS/Blueprints/Components/StatsManager/BP_StatsManagerComponent` (`self.GetComponentByClass` (`self.Gabriel`) "/Game/DynamicCombatSystem/DCS/Blueprints/Components/StatsManager/BP_StatsManagerComponent.BP_StatsManagerComponent_C")))
      (if (<= (`self.VidaMax`) 0.0)
        (bind _value (`/Game/DynamicCombatSystem/DCS/Blueprints/Components/StatsManager/BP_StatsManagerComponent.GetStatValue` _asbp_stats_manager_component (`BlueprintGameplayTagLibrary.MakeLiteralGameplayTag` (struct :`TagName` "Stat.Health.Current")) true))
        (set `self.VidaMax` _value))
      (if (and (not (`self.Empezado`)) (< (`KismetMathLibrary.Vector_Distance` (`self.K2_GetActorLocation` _returnvalue) (`self.K2_GetActorLocation` (`self.Gabriel`))) (`self.RadioArranque`)))
        (set `self.Empezado` true)
        (set `self.Fase` 1)
        (set `self.RespuestaCorrecta` 0)
        (set `self.PreguntaActiva` true)
        (`KismetSystemLibrary.PrintString` "GABRIEL: Que te trae al Reino?"))
      (bind _returnvalue_2 (/ _value (`KismetMathLibrary.FMax` (`self.VidaMax`) 1.0)))
      (if (and (== (`self.Fase`) 1) (<= _returnvalue_2 0.7))
        (set `self.Fase` 2)
        (`self.EncogerLaberinto`)
        (set `self.RespuestaCorrecta` 2)
        (set `self.PreguntaActiva` true)
        (`KismetSystemLibrary.PrintString` "GABRIEL: A quien sirves? - el laberinto encoge"))
      (if (and (== (`self.Fase`) 2) (<= _returnvalue_2 0.4))
        (set `self.Fase` 3)
        (set `self.PreguntaActiva` false)
        (`self.RomperEspejos`)
        (`KismetSystemLibrary.PrintString` "GABRIEL: Las Puertas no se abren para el penitente - los espejos estallan"))
      (bind _returnvalue_3 (- (`self.VidaAnterior`) _value))
      (if (and (== (`self.Fase`) 3) (and (and (> _returnvalue_3 1.0) (< _returnvalue_3 (`self.GolpeMaximo`))) (< (`KismetMathLibrary.Vector_Distance2D` (`self.K2_GetActorLocation` _returnvalue) (+ (`self.K2_GetActorLocation` (`self.Gabriel`)) (`self.OffsetSombra`))) (`self.RadioSombra`))))
        (bind _returnvalue_4 (- _value (* 0.5 _returnvalue_3)))
        (`/Game/DynamicCombatSystem/DCS/Blueprints/Components/StatsManager/BP_StatsManagerComponent.SetStat` _asbp_stats_manager_component (`BlueprintGameplayTagLibrary.MakeLiteralGameplayTag` (struct :`TagName` "Stat.Health.Current")) _returnvalue_4)
        (set `self.VidaAnterior` _returnvalue_4)
        (`KismetSystemLibrary.PrintString` "GOLPE SOBRE LA SOMBRA - 50 por ciento extra")
        (else
          (set `self.VidaAnterior` _value))))
    (:`Is Not Valid`
      (`self.RecogerEspejos`))))