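; BP_DA_RespuestaGabriel is an interactable answer option for the Gabriel boss fight.
; On Interact, it finds the BP_DA_GabrielFight actors in the level, records its mark name and strength on each, then calls Responder with its answer index.
; GetInteractionMessage returns the option's own text as the prompt, so the answer logic itself stays in the fight actor.
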(event `/Game/DynamicCombatSystem/DCS/Blueprints/Interfaces/I_IsInteractable.Interact`
  (params (Caller :type "Actor Object Reference"))
  (bind _outactors (`GameplayStatics.GetAllActorsOfClass` "/Game/DarkAngels/Blueprints/Bosses/BP_DA_GabrielFight.BP_DA_GabrielFight_C"))
  (for _array_element _outactors
    (bind _asbp_da_gabriel_fight (cast `/Game/DarkAngels/Blueprints/Bosses/BP_DA_GabrielFight` _array_element))
    (`/Game/DarkAngels/Blueprints/Bosses/BP_DA_GabrielFight.AnotarMarcaGabriel` _asbp_da_gabriel_fight (`self.Fuerza`) (`self.Marca`))
    (`/Game/DarkAngels/Blueprints/Bosses/BP_DA_GabrielFight.Responder` _asbp_da_gabriel_fight (`self.Indice`))))

(fn `GetInteractionMessage`
  (returns (Message :type Name))
  (return (`self.Texto`)))

(fn `UserConstructionScript`
  (`parent.UserConstructionScript`))