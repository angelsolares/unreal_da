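; Behavior tree task for Dark Angels boss AI that makes the controlled pawn chase the first player's pawn.
; On execute it runs AI MoveTo with the player as target actor and a close, fixed acceptance radius, then finishes as success or failure to match the move result.
; Three unconnected MoveTo variants with other radii, one randomized at longer range, remain in the graph but never run.
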(event `self.ReceiveExecuteAI`
  (params (OwnerController :type "AIController Object Reference") (ControlledPawn :type "Pawn Object Reference"))
  (`|AIMoveTo` ControlledPawn (`Actor.K2_GetActorLocation` (`GameplayStatics.GetPlayerPawn` 0)) (`GameplayStatics.GetPlayerPawn` 0) 145.0
    (:`OnSuccess`
      (`self.FinishExecute` true))
    (:`OnFail`
      (`self.FinishExecute` false))))