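; Behavior tree service that picks the boss's state from its distance to the player pawn.
; Each AI tick writes a blackboard enum with one of three states for far, mid-range or close.
; The current state selects the thresholds, giving hysteresis: the close state begins at a short range and holds until the player is about twice as far away.
; Disconnected alternative threshold checks, some randomized, never run.
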(event `self.ReceiveTickAI`
  (params (OwnerController :type "AIController Object Reference") (ControlledPawn :type "Pawn Object Reference") (DeltaSeconds :type "Float (single-precision)"))
  (bind _returnvalue (`AIBlueprintHelperLibrary.GetBlackboard` ControlledPawn))
  (bind _keyname (`self.KeyName`))
  (bind _returnvalue_2 (`BlackboardComponent.GetValueAsEnum` _returnvalue _keyname))
  (bind _returnvalue_3 (`KismetMathLibrary.VSize` (- (`Actor.K2_GetActorLocation` ControlledPawn) (`Actor.K2_GetActorLocation` (`GameplayStatics.GetPlayerPawn` 0)))))
  (if (== _returnvalue_2 2)
    (if (>= _returnvalue_3 9000.0)
      (`BlackboardComponent.SetValueAsEnum` _returnvalue _keyname 0)
      (elif (>= _returnvalue_3 700.0)
        (`BlackboardComponent.SetValueAsEnum` _returnvalue _keyname 1)))
    (elif (== _returnvalue_2 1)
      (if (>= _returnvalue_3 9000.0)
        (`BlackboardComponent.SetValueAsEnum` _returnvalue _keyname 0)
        (elif (<= _returnvalue_3 350.0)
          (`BlackboardComponent.SetValueAsEnum` _returnvalue _keyname 2)))
      (elif (<= _returnvalue_3 350.0)
        (`BlackboardComponent.SetValueAsEnum` _returnvalue _keyname 2)
        (elif (< _returnvalue_3 9000.0)
          (`BlackboardComponent.SetValueAsEnum` _returnvalue _keyname 1)
          (else
            (`BlackboardComponent.SetValueAsEnum` _returnvalue _keyname 0)))))))