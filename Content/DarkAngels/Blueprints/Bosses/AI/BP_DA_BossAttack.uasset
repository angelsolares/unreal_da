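; Behavior tree task that runs the attack of the BP_Giant boss.
; It turns the boss's yaw toward player 0, then plays a random montage from a short-range or long-range list, depending on the distance to the player.
; The task always finishes as failed, whether the montage completes or is interrupted.
; Two disconnected copies of the logic, which lack the turn and report success on completion, never run.
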(event `self.ReceiveExecuteAI`
  (params (OwnerController :type "AIController Object Reference") (ControlledPawn :type "Pawn Object Reference"))
  (bind _returnvalue (`Actor.K2_GetActorLocation` (`GameplayStatics.GetPlayerPawn` 0)))
  (bind _asbp_giant (cast `/Game/GiantBossProject/Blueprint/BP_Giant` ControlledPawn)
    (:`then`
      (bind _returnvalue_2 (`Actor.K2_GetActorLocation` _asbp_giant))
      (`Actor.K2_SetActorRotation` _asbp_giant (`KismetMathLibrary.MakeRotator` 0.0 0.0 (.yaw (`KismetMathLibrary.FindLookAtRotation` _returnvalue_2 _returnvalue))) false)
      (set `self.intermediate_distance` (`KismetMathLibrary.VSize` (- _returnvalue_2 _returnvalue)))
      (if (<= (`self.intermediate_distance`) 700.0)
        (bind _mesh (`Character.Mesh` _asbp_giant))
        (`|PlayMontage` _mesh (`KismetArrayLibrary.Array_Random` (`self.Montage to Play_Short`))
          (:`OnCompleted`
            (`self.FinishExecute` false))
          (:`OnInterrupted`
            (`self.FinishExecute` false)))
        (else
          (`|PlayMontage` _mesh (`KismetArrayLibrary.Array_Random` (`self.Montage to Play_Long`))
            (:`OnCompleted`
              (`self.FinishExecute` false))
            (:`OnInterrupted`
              (`self.FinishExecute` false))))))
    (:`CastFailed`
      (`self.FinishExecute` false))))