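; BP_DA_Inspector is an enemy Blueprint that can always be backstabbed and overrides montage selection and block rules from its parent.
; Montage lookup uses the parent's result when valid, otherwise falling back to the one-handed AI montage table.
; Blocking requires the block-input activity and a matching StateManager state, and is denied when the player's BP_DA_Vetas component reports Masacre.
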(fn `CanBeBackstabbed`
  (returns (ReturnValue :type Boolean))
  (return true))

(fn `CanBlock`
  (returns (ReturnValue :type Boolean))
  (bind _returnvalue (and (`/Game/DynamicCombatSystem/DCS/Blueprints/Components/StateManager/BP_StateManagerComponent.HasActivity` (`self.StateManager`) (struct :`GameplayTags` (struct :`(TagName` "Activity.IsBlockInputPressed") :`(TagName` "Activity.IsInCombat"))) "NewEnumerator1") (`/Game/DynamicCombatSystem/DCS/Blueprints/Components/StateManager/BP_StateManagerComponent.IsInState` (`self.StateManager`) "NewEnumerator1")))
  (bind _asbp_da_vetas (cast `/Game/DarkAngels/Blueprints/Combat/BP_DA_Vetas` (`self.GetComponentByClass` (`GameplayStatics.GetPlayerPawn` 0) "/Game/DarkAngels/Blueprints/Combat/BP_DA_Vetas.BP_DA_Vetas_C")))
  (`/Engine/EditorBlueprintResources/StandardMacros.IsValid` _asbp_da_vetas
    (:`Is Valid`
      (bind _valor (`/Game/DarkAngels/Blueprints/Combat/BP_DA_Vetas.TieneMasacre` _asbp_da_vetas))
      (return (and _returnvalue (not _valor))))
    (:`Is Not Valid`
      (return _returnvalue))))

(fn `GetMontages`
  (params (ActionTag :type "GameplayTag Structure"))
  (returns (Montages :type "DataTable Object Reference"))
  (bind _montages (`parent.GetMontages` ActionTag))
  (`/Engine/EditorBlueprintResources/StandardMacros.IsValid` _montages
    (:`Is Valid`
      (return _montages))
    (:`Is Not Valid`
      (return "/Game/DynamicCombatSystem/DCS/DataTables/Montages/AI/DT_AI_1H_Montages.DT_AI_1H_Montages"))))

(fn `UserConstructionScript`
  (`parent.UserConstructionScript`))