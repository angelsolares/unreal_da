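; Gabriel boss that wakes on proximity or damage and runs three HP-driven phases from Tick timers, without calling parent Tick.
; Phase 1 periodically tests player Farsa, dealing damage or removing mirrors.
; Phase 2 culls mirrors, spawns a Messenger, drains Farsa near mirrors and begins melee chase; phase 3 destroys mirrors, adding beams and a heavy-hit-breakable shield.
; AnyDamage handles shield, salt crystallization and death, which unlocks wings and raises Corruptio.
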(event `self.ReceiveBeginPlay`
  (`parent.ReceiveBeginPlay`))

(event `self.ReceiveActorBeginOverlap`
  (params (OtherActor :type "Actor Object Reference"))
  (`parent.ReceiveActorBeginOverlap` OtherActor))

(event `self.ReceiveTick`
  (params (DeltaSeconds :type "Float (single-precision)"))
  (bind _returnvalue (`GameplayStatics.GetPlayerCharacter` 0))
  (bind _returnvalue_2 (`self.K2_GetActorLocation`))
  (bind _returnvalue_3 (`self.K2_GetActorLocation` _returnvalue))
  (bind _returnvalue_4 (`KismetMathLibrary.Vector_Distance` _returnvalue_2 _returnvalue_3))
  (set `self.AttackCooldown` (- (`self.AttackCooldown`) DeltaSeconds))
  (set `self.BeamTimer` (- (`self.BeamTimer`) DeltaSeconds))
  (set `self.ShieldTimer` (- (`self.ShieldTimer`) DeltaSeconds))
  (set `self.QuestionTimer` (- (`self.QuestionTimer`) DeltaSeconds))
  (set `self.ShieldRegenTimer` (- (`self.ShieldRegenTimer`) DeltaSeconds))
  (if (`self.bDormant`)
    (if (< _returnvalue_4 2000.0)
      (set `self.bDormant` false)
      (set `self.QuestionTimer` 5.0)
      (`KismetSystemLibrary.PrintString` "GABRIEL - Phase 1: THE LABYRINTH"))
    (else
      (if (and (<= (`self.HP`) 560.0) (not (`self.bPhase2Triggered`)))
        (set `self.bPhase2Triggered` true)
        (set `self.Phase` 2)
        (`KismetSystemLibrary.PrintString` "PHASE 2 - THE DOUBT: the labyrinth shrinks")
        (set `self.MirrorsDestroyed` 0)
        (bind _outactors (`GameplayStatics.GetAllActorsWithTag` "Mirror"))
        (for _array_element _outactors
          (if (< (`self.MirrorsDestroyed`) 4)
            (`self.K2_DestroyActor` _array_element)
            (set `self.MirrorsDestroyed` (+ (`self.MirrorsDestroyed`) 1))))
        (`|SpawnActorFromClass` "/Game/DarkAngels/Blueprints/Enemies/BP_Angel_Messenger.BP_Angel_Messenger_C" (`KismetMathLibrary.MakeTransform` (+ _returnvalue_2 (`KismetMathLibrary.MakeVector` 250.0 0.0 20.0))) "AlwaysSpawn" "MultiplyWithRoot" null null))
      (if (and (<= (`self.HP`) 280.0) (not (`self.bPhase3Triggered`)))
        (set `self.bPhase3Triggered` true)
        (set `self.Phase` 3)
        (`KismetSystemLibrary.PrintString` "PHASE 3 - THE JUDGMENT: all mirrors destroyed")
        (bind _outactors_2 (`GameplayStatics.GetAllActorsWithTag` "Mirror"))
        (for _array_element_2 _outactors_2
          (`self.K2_DestroyActor` _array_element_2)))
      (if (== (`self.Phase`) 1)
        (if (<= (`self.QuestionTimer`) 0.0)
          (set `self.QuestionTimer` 10.0)
          (set `self.QuestionIndex` (+ (`self.QuestionIndex`) 1))
          (bind _asbp_da_player_character_v2 (cast `/Game/DarkAngels/Blueprints/Characters/BP_DA_PlayerCharacter_V2` _returnvalue))
          (if (< (`/Game/DarkAngels/Blueprints/Characters/BP_DA_PlayerCharacter_V2.Farsa` _asbp_da_player_character_v2) 50.0)
            (`KismetSystemLibrary.PrintString` "Gabriel: YOUR SHADOW IS TOO LONG - all traps activate")
            (`GameplayStatics.ApplyDamage` _returnvalue 25.0 null self)
            (else
              (`KismetSystemLibrary.PrintString` "Gabriel asks. Humble answer: PROCEED - mirror path opens")
              (set `self.MirrorsDestroyed` 0)
              (bind _outactors_3 (`GameplayStatics.GetAllActorsWithTag` "Mirror"))
              (for _array_element_3 _outactors_3
                (if (< (`self.MirrorsDestroyed`) 2)
                  (`self.K2_DestroyActor` _array_element_3)
                  (set `self.MirrorsDestroyed` (+ (`self.MirrorsDestroyed`) 1))))))
          (else
            (if (== (`self.Phase`) 2) :!label _label
              (bind _outactors_4 (`GameplayStatics.GetAllActorsWithTag` "Mirror"))
              (set `self.bNearMirror` false)
              (for _array_element_4 _outactors_4
                (if (< (`KismetMathLibrary.Vector_Distance` _returnvalue_3 (`self.K2_GetActorLocation` _array_element_4)) 600.0)
                  (set `self.bNearMirror` true)))
              (if (`self.bNearMirror`)
                (set `self.GazeTimer` (+ (`self.GazeTimer`) DeltaSeconds))
                (else
                  (set `self.GazeTimer` 0.0)))
              (if (> (`self.GazeTimer`) 2.0)
                (bind _asbp_da_player_character_v2_2 (cast `/Game/DarkAngels/Blueprints/Characters/BP_DA_PlayerCharacter_V2` _returnvalue))
                (bind _farsa (`/Game/DarkAngels/Blueprints/Characters/BP_DA_PlayerCharacter_V2.Farsa` _asbp_da_player_character_v2_2))
                (set `/Game/DarkAngels/Blueprints/Characters/BP_DA_PlayerCharacter_V2.Farsa` (select `bool` (< (- _farsa (* 5.0 DeltaSeconds)) 0.0) :`false` (- _farsa (* 5.0 DeltaSeconds)) :`true` 0.0) _asbp_da_player_character_v2_2)
                (`KismetSystemLibrary.PrintString` "Mirror gaze drains Farsa - black wings reflection")
                (else
                  (if (>= (`self.Phase`) 2) :!label _label_2
                    (if (> _returnvalue_4 250.0)
                      (`self.AddMovementInput` (`KismetMathLibrary.Vector_NormalUnsafe` (- _returnvalue_3 _returnvalue_2))))
                    (if (and (< _returnvalue_4 300.0) (<= (`self.AttackCooldown`) 0.0))
                      (`KismetSystemLibrary.PrintString` "Gabriel heavy swing")
                      (`GameplayStatics.ApplyDamage` _returnvalue (`self.Damage`) null self)
                      (set `self.AttackCooldown` 2.5))
                    (if (== (`self.Phase`) 3)
                      (if (<= (`self.BeamTimer`) 0.0)
                        (set `self.BeamTimer` 12.0)
                        (`|SpawnActorFromClass` "/Game/DarkAngels/Blueprints/World/BP_DA_BeamVisual.BP_DA_BeamVisual_C" (`KismetMathLibrary.MakeTransform` _returnvalue_3) "AlwaysSpawn" "MultiplyWithRoot" null null)
                        (`GameplayStatics.ApplyDamage` _returnvalue 20.0 null self)
                        (`KismetSystemLibrary.PrintString` "GABRIEL JUDGMENT BEAM"))
                      (if (<= (`self.ShieldRegenTimer`) 0.0)
                        (set `self.ShieldRegenTimer` 15.0)
                        (if (not (`self.bShieldUp`))
                          (set `self.bShieldUp` true)
                          (set `self.ShieldHits` 0)
                          (set `self.ShieldTimer` 5.0)
                          (`|SpawnActorFromClass` "/Game/DarkAngels/Blueprints/Enemies/BP_LightShield.BP_LightShield_C" (`KismetMathLibrary.MakeTransform` _returnvalue_2) "AlwaysSpawn" "MultiplyWithRoot" null null)
                          (`KismetSystemLibrary.PrintString` "Gabriel Light Shield regenerates")))))
                  (if (and (`self.bShieldUp`) (<= (`self.ShieldTimer`) 0.0))
                    (set `self.bShieldUp` false)
                    (bind _outactors_5 (`GameplayStatics.GetAllActorsWithTag` "LightShield"))
                    (for _array_element_5 _outactors_5
                      (`self.K2_DestroyActor` _array_element_5)))))
              (else
                (goto _label_2)))))
        (else
          (goto _label))))))

(event `self.ReceiveAnyDamage`
  (params (Damage :type "Float (single-precision)") (DamageType :type "DamageType Object Reference") (InstigatedBy :type "Controller Object Reference") (DamageCauser :type "Actor Object Reference"))
  (if (`self.bDormant`)
    (set `self.bDormant` false)
    (set `self.QuestionTimer` 5.0))
  (if (`self.bShieldUp`)
    (if (>= Damage 60.0)
      (set `self.ShieldHits` (+ (`self.ShieldHits`) 1))
      (`KismetSystemLibrary.PrintString` "Dark Strike hit Gabriel shield")
      (if (>= (`self.ShieldHits`) 3)
        (set `self.bShieldUp` false)
        (set `self.ShieldTimer` 0.0)
        (bind _outactors (`GameplayStatics.GetAllActorsWithTag` "LightShield"))
        (for _array_element _outactors
          (`self.K2_DestroyActor` _array_element))
        (`KismetSystemLibrary.PrintString` "GABRIEL SHIELD BREAK"))
      (else
        (`KismetSystemLibrary.PrintString` "Blocked by Gabriel Light Shield")))
    (else
      (set `self.HP` (- (`self.HP`) Damage))
      (if (and (<= (`self.HP`) 80.0) (not (`self.bCrystallizing`)))
        (set `self.bCrystallizing` true)
        (`PrimitiveComponent.SetMaterial` (`self.BodyMesh`) 0 "/Game/DarkAngels/Materials/Malkuth/M_DA_MK_Salt_Crystal.M_DA_MK_Salt_Crystal")
        (`KismetSystemLibrary.PrintString` "Gabriel kneels - crystallizing into salt"))
      (if (<= (`self.HP`) 0.0)
        (`KismetSystemLibrary.PrintString` "GABRIEL DEFEATED - crumbles to dust. WINGS UNLOCKED")
        (bind _asbp_da_player_character_v2 (cast `/Game/DarkAngels/Blueprints/Characters/BP_DA_PlayerCharacter_V2` (`GameplayStatics.GetPlayerCharacter` 0))
          (:`then`
            (set `/Game/DarkAngels/Blueprints/Characters/BP_DA_PlayerCharacter_V2.bWingsUnlocked` true _asbp_da_player_character_v2)
            (bind _returnvalue (+ (`/Game/DarkAngels/Blueprints/Characters/BP_DA_PlayerCharacter_V2.Corruptio` _asbp_da_player_character_v2) 15.0))
            (set `/Game/DarkAngels/Blueprints/Characters/BP_DA_PlayerCharacter_V2.Corruptio` (select `bool` (> _returnvalue 100.0) :`false` _returnvalue :`true` 100.0) _asbp_da_player_character_v2)
            (`self.K2_DestroyActor` self))
          (:`CastFailed`
            (`self.K2_DestroyActor` self)))))))

(fn `UserConstructionScript`
  (`parent.UserConstructionScript`))