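; Archangel boss enemy that wakes on player proximity or damage, then chases and melees the player.
; Tick runs cooldowns and HP-based phases: phase 2 adds an unavoidable beam, phase 3 adds Messenger summons and higher movement input.
; A one-time timed Light Shield blocks damage until expiry or three heavy hits, with visuals removed by tag.
; Death raises player Corruptio, capped; PrintString stands in for combat feedback.
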(event `self.ReceiveTick`
  (params (DeltaSeconds :type "Float (single-precision)"))
  (bind _returnvalue (`GameplayStatics.GetPlayerCharacter` 0))
  (bind _returnvalue_2 (`self.K2_GetActorLocation`))
  (bind _returnvalue_3 (`self.K2_GetActorLocation` _returnvalue))
  (bind _returnvalue_4 (`KismetMathLibrary.Vector_Distance` _returnvalue_2 _returnvalue_3))
  (set `self.AttackCooldown` (- (`self.AttackCooldown`) DeltaSeconds))
  (set `self.BeamTimer` (- (`self.BeamTimer`) DeltaSeconds))
  (set `self.SummonTimer` (- (`self.SummonTimer`) DeltaSeconds))
  (set `self.ShieldTimer` (- (`self.ShieldTimer`) DeltaSeconds))
  (if (`self.bDormant`)
    (if (< _returnvalue_4 1500.0)
      (set `self.bDormant` false)
      (`KismetSystemLibrary.PrintString` "Archangel awakened"))
    (else
      (if (and (`self.bShieldUp`) (<= (`self.ShieldTimer`) 0.0))
        (set `self.bShieldUp` false)
        (bind _outactors (`GameplayStatics.GetAllActorsWithTag` "LightShield"))
        (for _array_element _outactors
          (`self.K2_DestroyActor` _array_element))
        (`KismetSystemLibrary.PrintString` "Light Shield expired"))
      (if (> (`self.HP`) 280.0)
        (set `self.Phase` 1)
        (elif (> (`self.HP`) 160.0)
          (set `self.Phase` 2)
          (else
            (set `self.Phase` 3))))
      (if (== (`self.Phase`) 3)
        (if (not (`self.bPhase3`))
          (set `self.bPhase3` true)
          (`KismetSystemLibrary.PrintString` "Archangel Phase 3 - desperation speed"))
        (if (<= (`self.SummonTimer`) 0.0)
          (set `self.SummonTimer` 20.0)
          (`|SpawnActorFromClass` "/Game/DarkAngels/Blueprints/Enemies/BP_Angel_Messenger.BP_Angel_Messenger_C" (`KismetMathLibrary.MakeTransform` (+ _returnvalue_2 (`KismetMathLibrary.MakeVector` 200.0 0.0 20.0))) "AlwaysSpawn" "MultiplyWithRoot" null null)
          (`KismetSystemLibrary.PrintString` "Archangel summons Messenger")))
      (if (> _returnvalue_4 220.0)
        (`self.AddMovementInput` (`KismetMathLibrary.Vector_NormalUnsafe` (- _returnvalue_3 _returnvalue_2)) (select `bool` (== (`self.Phase`) 3) :`false` 1.0 :`true` 1.2)))
      (if (and (< _returnvalue_4 280.0) (<= (`self.AttackCooldown`) 0.0))
        (`KismetSystemLibrary.PrintString` "Archangel heavy swing - sword glow telegraph")
        (`GameplayStatics.ApplyDamage` _returnvalue (`self.Damage`) null self)
        (set `self.AttackCooldown` 2.5))
      (if (>= (`self.Phase`) 2)
        (if (<= (`self.BeamTimer`) 0.0)
          (set `self.BeamTimer` 12.0)
          (`|SpawnActorFromClass` "/Game/DarkAngels/Blueprints/World/BP_DA_BeamVisual.BP_DA_BeamVisual_C" (`KismetMathLibrary.MakeTransform` _returnvalue_3) "AlwaysSpawn" "MultiplyWithRoot" null null)
          (`GameplayStatics.ApplyDamage` _returnvalue 20.0 null self)
          (`KismetSystemLibrary.PrintString` "JUDGMENT BEAM - thunderclap"))))))

(event `self.ReceiveAnyDamage`
  (params (Damage :type "Float (single-precision)") (DamageType :type "DamageType Object Reference") (InstigatedBy :type "Controller Object Reference") (DamageCauser :type "Actor Object Reference"))
  (if (`self.bDormant`)
    (set `self.bDormant` false))
  (if (`self.bShieldUp`)
    (if (>= Damage 60.0)
      (set `self.ShieldHits` (+ (`self.ShieldHits`) 1))
      (`KismetSystemLibrary.PrintString` "Dark Strike hit shield")
      (if (>= (`self.ShieldHits`) 3)
        (set `self.bShieldUp` false)
        (set `self.ShieldTimer` 0.0)
        (bind _outactors (`GameplayStatics.GetAllActorsWithTag` "LightShield"))
        (for _array_element _outactors
          (`self.K2_DestroyActor` _array_element))
        (`KismetSystemLibrary.PrintString` "LIGHT SHIELD BREAK - glass shatter"))
      (else
        (`KismetSystemLibrary.PrintString` "Blocked by Light Shield")))
    (else
      (set `self.HP` (- (`self.HP`) Damage))
      (if (and (< (`self.HP`) 280.0) (not (`self.bShieldUsed`)))
        (set `self.bShieldUsed` true)
        (set `self.bShieldUp` true)
        (set `self.ShieldHits` 0)
        (set `self.ShieldTimer` 5.0)
        (`|SpawnActorFromClass` "/Game/DarkAngels/Blueprints/Enemies/BP_LightShield.BP_LightShield_C" (`KismetMathLibrary.MakeTransform` (`self.K2_GetActorLocation`)) "AlwaysSpawn" "MultiplyWithRoot" null null)
        (`KismetSystemLibrary.PrintString` "Light Shield raised"))
      (if (<= (`self.HP`) 0.0)
        (`KismetSystemLibrary.PrintString` "Archangel death - feather dissolve")
        (bind _asbp_da_player_character_v2 (cast `/Game/DarkAngels/Blueprints/Characters/BP_DA_PlayerCharacter_V2` (`GameplayStatics.GetPlayerCharacter` 0))
          (:`then`
            (bind _returnvalue (+ (`/Game/DarkAngels/Blueprints/Characters/BP_DA_PlayerCharacter_V2.Corruptio` _asbp_da_player_character_v2) 15.0))
            (set `/Game/DarkAngels/Blueprints/Characters/BP_DA_PlayerCharacter_V2.Corruptio` (select `bool` (> _returnvalue 100.0) :`false` _returnvalue :`true` 100.0) _asbp_da_player_character_v2)
            (`self.K2_DestroyActor` self))
          (:`CastFailed`
            (`self.K2_DestroyActor` self)))))))

(fn `UserConstructionScript`)