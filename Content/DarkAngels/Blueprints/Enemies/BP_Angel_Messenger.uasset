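; Messenger angel enemy that patrols points and turns hostile when the player's Farsa drops low or it takes damage.
; Tick runs a string state machine: patrol tilts the head near high-Farsa players, attack chases and deals cooldown-gated melee damage.
; At low HP it spawns one copy of itself; trumpet stun is only a timed print.
; Death raises player Corruptio and damages a nearby player if any Archangel-tagged actor exists.
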(event `self.ReceiveBeginPlay`
  (set `self.State` "Patrol"))

(event `self.ReceiveTick`
  (params (DeltaSeconds :type "Float (single-precision)"))
  (bind _returnvalue (`GameplayStatics.GetPlayerCharacter` 0))
  (bind _returnvalue_2 (`self.K2_GetActorLocation`))
  (bind _returnvalue_3 (`KismetArrayLibrary.Array_Length` (`self.PatrolPoints`)))
  (bind _returnvalue_4 (`self.K2_GetActorLocation` _returnvalue))
  (bind _output (`|GetArrayItem` (`self.PatrolPoints`) (`self.PatrolIndex`)))
  (bind _returnvalue_5 (`KismetMathLibrary.Vector_Distance` _returnvalue_2 _returnvalue_4))
  (set `self.AttackCooldown` (- (`self.AttackCooldown`) DeltaSeconds))
  (set `self.TrumpetTimer` (- (`self.TrumpetTimer`) DeltaSeconds))
  (bind _asbp_da_player_character_v2 (cast `/Game/DarkAngels/Blueprints/Characters/BP_DA_PlayerCharacter_V2` _returnvalue))
  (bind _farsa (`/Game/DarkAngels/Blueprints/Characters/BP_DA_PlayerCharacter_V2.Farsa` _asbp_da_player_character_v2))
  (set `self.PlayerFarsa` _farsa)
  (if (== (`self.State`) "Patrol")
    (if (> _returnvalue_3 0)
      (if (>= (`self.PatrolIndex`) _returnvalue_3)
        (set `self.PatrolIndex` 0))
      (if (< (`KismetMathLibrary.Vector_Distance` _returnvalue_2 _output) 120.0)
        (set `self.PatrolIndex` (+ (`self.PatrolIndex`) 1))
        (else
          (`self.AddMovementInput` (`KismetMathLibrary.Vector_NormalUnsafe` (- _output _returnvalue_2)) 1.0))))
    (if (and (< _returnvalue_5 1000.0) (> _farsa 70.0))
      (`SceneComponent.K2_SetRelativeRotation` (`self.HeadMesh`) (`KismetMathLibrary.MakeRotator` 15.0) false false)
      (else
        (`SceneComponent.K2_SetRelativeRotation` (`self.HeadMesh`) (`KismetMathLibrary.MakeRotator` 0.0) false false)))
    (if (< _farsa 40.0)
      (set `self.State` "Attack")))
  (if (== (`self.State`) "Attack")
    (if (> _returnvalue_5 180.0)
      (`self.AddMovementInput` (`KismetMathLibrary.Vector_NormalUnsafe` (- _returnvalue_4 _returnvalue_2)) 1.0))
    (if (and (< _returnvalue_5 220.0) (<= (`self.AttackCooldown`) 0.0))
      (`GameplayStatics.ApplyDamage` _returnvalue (`self.Damage`) null self)
      (set `self.AttackCooldown` 1.2))
    (if (<= (`self.TrumpetTimer`) 0.0)
      (`KismetSystemLibrary.PrintString` "TRUMPET STUN - player stunned 0.8s")
      (set `self.TrumpetTimer` 8.0))
    (if (and (< (`self.HP`) 30.0) (not (`self.bReinforcementCalled`)))
      (set `self.bReinforcementCalled` true)
      (`|SpawnActorFromClass` "BP_Angel_Messenger_C" (`KismetMathLibrary.MakeTransform` (+ _returnvalue_2 (`KismetMathLibrary.MakeVector` 150.0 0.0 20.0))) "AlwaysSpawn" "MultiplyWithRoot" null null))))

(event `self.ReceiveAnyDamage`
  (params (Damage :type "Float (single-precision)") (DamageType :type "DamageType Object Reference") (InstigatedBy :type "Controller Object Reference") (DamageCauser :type "Actor Object Reference"))
  (bind _returnvalue (`GameplayStatics.GetPlayerCharacter` 0))
  (set `self.HP` (- (`self.HP`) Damage))
  (set `self.State` "Attack")
  (if (<= (`self.HP`) 0.0)
    (`KismetSystemLibrary.PrintString` "Angel Messenger death - feather dissolve")
    (bind _asbp_da_player_character_v2 (cast `/Game/DarkAngels/Blueprints/Characters/BP_DA_PlayerCharacter_V2` _returnvalue)
      (:`then`
        (bind _returnvalue_2 (+ (`/Game/DarkAngels/Blueprints/Characters/BP_DA_PlayerCharacter_V2.Corruptio` _asbp_da_player_character_v2) 15.0))
        (set `/Game/DarkAngels/Blueprints/Characters/BP_DA_PlayerCharacter_V2.Corruptio` (select `bool` (> _returnvalue_2 100.0) :`false` _returnvalue_2 :`true` 100.0) _asbp_da_player_character_v2)
        (bind _outactors (`GameplayStatics.GetAllActorsWithTag` "Archangel"))
        (if (> (`KismetArrayLibrary.Array_Length` _outactors) 0)
          (if (< (`KismetMathLibrary.Vector_Distance` (`self.K2_GetActorLocation`) (`self.K2_GetActorLocation` _returnvalue)) 300.0)
            (`GameplayStatics.ApplyDamage` _returnvalue 30.0 null self)
            (`KismetSystemLibrary.PrintString` "DESPERATION self-destruct")))
        (`self.K2_DestroyActor` self))
      (:`CastFailed`
        (`self.K2_DestroyActor` self)))))

(fn `UserConstructionScript`)