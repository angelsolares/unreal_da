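; Component that changes the "Intensidad" material parameter on its owner's skeletal mesh as a proximity cue, likely a glowing face.
; On BeginPlay it creates a dynamic material instance on element 0 and starts the looping Latir timer instead of using Tick.
; Latir eases the value toward IntensidadMax while the player character is within RadioAviso, otherwise toward IntensidadBase, using FInterpTo with a fixed step matching the timer.
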(event `self.ReceiveBeginPlay`
  (bind _asskeletal_mesh_component (cast `SkeletalMeshComponent` (`Actor.GetComponentByClass` (`self.GetOwner`) "/Script/Engine.SkeletalMeshComponent")))
  (bind _returnvalue (`PrimitiveComponent.CreateDynamicMaterialInstance` _asskeletal_mesh_component 0 null "None"))
  (set `self.MID` _returnvalue)
  (`KismetSystemLibrary.K2_SetTimer` self "Latir" 0.1 true))

(fn `Latir`
  (`/Engine/EditorBlueprintResources/StandardMacros.IsValid` (`self.MID`)
    (:`Is Valid`
      (set `self.Actual` (`KismetMathLibrary.FInterpTo` (`self.Actual`) (select `bool` (< (`KismetMathLibrary.Vector_Distance` (`Actor.K2_GetActorLocation` (`self.GetOwner`)) (`Actor.K2_GetActorLocation` (`GameplayStatics.GetPlayerCharacter` 0))) (`self.RadioAviso`)) :`false` (`self.IntensidadBase`) :`true` (`self.IntensidadMax`)) 0.1 4.0))
      (`MaterialInstanceDynamic.SetScalarParameterValue` (`self.MID`) "Intensidad" (`self.Actual`)))))