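; Anim notify state named TechWindow that marks the span of an animation during which the player character can tech roll.
; On begin it casts the mesh owner to BP_DA_PlayerCharacter and sets CanTechRoll true, then sets it false on end.
; Leftover collision handler activate and deactivate logic sits in both events but is disconnected and never runs.
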(fn `GetNotifyName`
  (returns (ReturnValue :type String))
  (return "TechWindow"))

(fn `Received_NotifyBegin`
  (params (MeshComp :type "SkeletalMeshComponent Object Reference") (Animation :type "AnimSequenceBase Object Reference") (TotalDuration :type "Float (single-precision)") (EventReference :type "AnimNotifyEventReference Structure (by ref)"))
  (returns (ReturnValue :type Boolean))
  (bind _asbp_da_player_character (cast `/Game/DarkAngels/Blueprints/Characters/BP_DA_PlayerCharacter` (`ActorComponent.GetOwner` MeshComp))
    (:`then`
      (set `/Game/DarkAngels/Blueprints/Characters/BP_DA_PlayerCharacter.CanTechRoll` true _asbp_da_player_character)
      (return true))
    (:`CastFailed`
      (return false))))

(fn `Received_NotifyEnd`
  (params (MeshComp :type "SkeletalMeshComponent Object Reference") (Animation :type "AnimSequenceBase Object Reference") (EventReference :type "AnimNotifyEventReference Structure (by ref)"))
  (returns (ReturnValue :type Boolean))
  (bind _asbp_da_player_character (cast `/Game/DarkAngels/Blueprints/Characters/BP_DA_PlayerCharacter` (`ActorComponent.GetOwner` MeshComp))
    (:`then`
      (set `/Game/DarkAngels/Blueprints/Characters/BP_DA_PlayerCharacter.CanTechRoll` false _asbp_da_player_character)
      (return true))
    (:`CastFailed`
      (return false))))