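; Component that shows the player's marks as corruption veins on the owner's skeletal mesh, using a dynamic material in slot 0.
; A looping Latir timer reads three force counts from BP_DA_GameState and eases the Corrupcion parameter toward their scaled total.
; Three vein colors fill in Gracia, Corrupcion, Voluntad order by count, with missing ranks repeating the last filled color.
; FijarBrillo sets vein glow separately.
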(event `self.ReceiveBeginPlay`
  (bind _asskeletal_mesh_component (cast `SkeletalMeshComponent` (`Actor.GetComponentByClass` (`self.GetOwner`) "/Script/Engine.SkeletalMeshComponent")))
  (`PrimitiveComponent.SetMaterial` _asskeletal_mesh_component 0 (`self.Material`))
  (bind _returnvalue (`PrimitiveComponent.CreateDynamicMaterialInstance` _asskeletal_mesh_component 0 null "None"))
  (set `self.MID` _returnvalue)
  (`KismetSystemLibrary.K2_SetTimer` self "Latir" 0.25 true))

(fn `FijarBrillo`
  (params (Valor :type "Float (double-precision)"))
  (bind _mid (`self.MID`))
  (`/Engine/EditorBlueprintResources/StandardMacros.IsValid` _mid
    (:`Is Valid`
      (`MaterialInstanceDynamic.SetScalarParameterValue` _mid "BrilloVena" Valor))))

(fn `Latir`
  (bind _asbp_da_game_state (cast `/Game/DarkAngels/Blueprints/World/BP_DA_GameState` (`GameplayStatics.GetGameState`)))
  (bind _cuantas (`/Game/DarkAngels/Blueprints/World/BP_DA_GameState.LeerFuerza` _asbp_da_game_state 1))
  (bind _cuantas_2 (`/Game/DarkAngels/Blueprints/World/BP_DA_GameState.LeerFuerza` _asbp_da_game_state 2))
  (bind _cuantas_3 (`/Game/DarkAngels/Blueprints/World/BP_DA_GameState.LeerFuerza` _asbp_da_game_state 3))
  (bind _returnvalue (+ (+ _cuantas _cuantas_2) _cuantas_3))
  (set `self.Actual` (`KismetMathLibrary.FInterpTo` (`self.Actual`) (* (`KismetMathLibrary.Conv_IntToDouble` _returnvalue) (`self.IntensidadPorMarca`)) 0.25 2.0))
  (`/Engine/EditorBlueprintResources/StandardMacros.IsValid` (`self.MID`)
    (:`Is Valid`
      (`MaterialInstanceDynamic.SetScalarParameterValue` (`self.MID`) "Corrupcion" (`self.Actual`))
      (bind _returnvalue_2 (select `bool` (>= _cuantas 1) :`false` (select `bool` (>= _cuantas_2 1) :`false` (`self.ColorVoluntad`) :`true` (`self.ColorCorrupcion`)) :`true` (`self.ColorGracia`)))
      (`MaterialInstanceDynamic.SetVectorParameterValue` (`self.MID`) "ColorVena" _returnvalue_2)
      (bind _returnvalue_3 (select `bool` (>= _returnvalue 2) :`false` _returnvalue_2 :`true` (select `bool` (>= _cuantas 2) :`false` (select `bool` (>= (+ _cuantas _cuantas_2) 2) :`false` (`self.ColorVoluntad`) :`true` (`self.ColorCorrupcion`)) :`true` (`self.ColorGracia`))))
      (`MaterialInstanceDynamic.SetVectorParameterValue` (`self.MID`) "ColorVena2" _returnvalue_3)
      (`MaterialInstanceDynamic.SetVectorParameterValue` (`self.MID`) "ColorVena3" (select `bool` (>= _returnvalue 3) :`false` _returnvalue_3 :`true` (select `bool` (>= _cuantas 3) :`false` (select `bool` (>= (+ _cuantas _cuantas_2) 3) :`false` (`self.ColorVoluntad`) :`true` (`self.ColorCorrupcion`)) :`true` (`self.ColorGracia`)))))))