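; BP_DA_DestelloDescarte is a short-lived visual flash actor, by its name for a discard in combat, showing an expanding ground ring with a blue light burst.
; On BeginPlay, Arrancar sets a sub-second lifespan and builds a collision-free plane and point light at runtime.
; A looping timer runs Latir, which linearly grows the plane and fades the light to zero based on elapsed time, without using Tick.
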(event `self.ReceiveBeginPlay`
  (`self.Arrancar`))

(fn `Arrancar`
  (`self.SetLifeSpan` self 0.8)
  (set `self.TNacio` (`KismetSystemLibrary.GetGameTimeInSeconds`))
  (bind _returnvalue (`|AddComponentByClass` :`self` self :`Class` "/Script/Engine.StaticMeshComponent"))
  (bind _asstatic_mesh_component (cast `StaticMeshComponent` _returnvalue))
  (set `self.Anillo` _asstatic_mesh_component)
  (`StaticMeshComponent.SetStaticMesh` (`self.Anillo`) "/Engine/BasicShapes/Plane.Plane")
  (`PrimitiveComponent.SetMaterial` (`self.Anillo`) 0 "/Game/DarkAngels/Materials/MI_DA_PilarArma.MI_DA_PilarArma")
  (`PrimitiveComponent.SetCollisionEnabled` (`self.Anillo`) "NoCollision")
  (`SceneComponent.K2_SetRelativeLocation` (`self.Anillo`) (`KismetMathLibrary.MakeVector` 0.0 0.0 12.0) false false)
  (`SceneComponent.SetRelativeScale3D` (`self.Anillo`) (`KismetMathLibrary.MakeVector` 0.8 0.8 1.0))
  (bind _returnvalue_2 (`|AddComponentByClass` :`self` self :`Class` "/Script/Engine.PointLightComponent"))
  (bind _aspoint_light_component (cast `PointLightComponent` _returnvalue_2))
  (set `self.LuzD` _aspoint_light_component)
  (`LightComponent.SetLightColor` (`self.LuzD`) (make `LinearColor` 0.3 0.62 1.0 1.0) true)
  (`LocalLightComponent.SetAttenuationRadius` (`self.LuzD`) 1200.0)
  (`LightComponent.SetIntensity` (`self.LuzD`) 25000.0)
  (`KismetSystemLibrary.K2_SetTimer` self "Latir" 0.02 true))

(fn `Latir`
  (bind _returnvalue (`KismetMathLibrary.FMin` 1.0 (/ (- (`KismetSystemLibrary.GetGameTimeInSeconds`) (`self.TNacio`)) 0.7)))
  (bind _returnvalue_2 (+ 0.8 (* 6.0 _returnvalue)))
  (`LightComponent.SetIntensity` (`self.LuzD`) (* 25000.0 (- 1.0 _returnvalue)))
  (`SceneComponent.SetRelativeScale3D` (`self.Anillo`) (`KismetMathLibrary.MakeVector` _returnvalue_2 _returnvalue_2 1.0)))

(fn `UserConstructionScript`)