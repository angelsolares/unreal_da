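; Animation notify state that applies a hit stop in combat by changing global time dilation during its window in an animation.
; NotifyBegin sets the world's dilation to the notify's Dilatacion value.
; NotifyEnd sets it to FinDilatacion, read from player 0's BP_DA_HUD; if that cast fails, dilation is left unchanged.
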(fn `Received_NotifyBegin`
  (params (MeshComp :type "SkeletalMeshComponent Object Reference") (Animation :type "AnimSequenceBase Object Reference") (TotalDuration :type "Float (single-precision)") (EventReference :type "AnimNotifyEventReference Structure (by ref)"))
  (returns (ReturnValue :type Boolean))
  (`GameplayStatics.SetGlobalTimeDilation` MeshComp (`self.Dilatacion`))
  (return false))

(fn `Received_NotifyEnd`
  (params (MeshComp :type "SkeletalMeshComponent Object Reference") (Animation :type "AnimSequenceBase Object Reference") (EventReference :type "AnimNotifyEventReference Structure (by ref)"))
  (returns (ReturnValue :type Boolean))
  (bind _asbp_da_hud (cast `/Game/DarkAngels/Blueprints/UI/BP_DA_HUD` (`PlayerController.GetHUD` (`GameplayStatics.GetPlayerController` MeshComp))))
  (`GameplayStatics.SetGlobalTimeDilation` MeshComp (`/Game/DarkAngels/Blueprints/UI/BP_DA_HUD.Fin_Dilatacion` _asbp_da_hud))
  (return false))