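; Dropped weapon pickup that records its source enemy and becomes the player's temporary weapon when interacted with.
; Caer runs a physics fall until low speed or a timeout triggers Posar, which snaps it to the ground and enables Zona.
; A runtime-built cone pillar and light pulse on Tick, sized and centered from mesh bounds.
; Interact swaps the temporary weapon, schedules its corruption, adds and equips the item, then destroys the actor.
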(event `self.ReceiveBeginPlay`
  (`parent.ReceiveBeginPlay`)
  (`self.MontarPilar`))

(event `/Game/DynamicCombatSystem/DCS/Blueprints/Interfaces/I_IsInteractable.Interact`
  (params (Caller :type "Actor Object Reference"))
  (bind _itemalrecoger (`self.ItemAlRecoger`))
  (`self.OcultarCartel` Caller)
  (`/Engine/EditorBlueprintResources/StandardMacros.IsValid` _itemalrecoger
    (:`Is Valid`
      (`self.CanjearTemporal` Caller _itemalrecoger)
      (bind _asbp_inventory_component (cast `/Game/DynamicCombatSystem/DCS/Blueprints/Components/Inventory/BP_InventoryComponent` (`self.GetComponentByClass` Caller "/Game/DynamicCombatSystem/DCS/Blueprints/Components/Inventory/BP_InventoryComponent.BP_InventoryComponent_C")))
      (`/Game/DynamicCombatSystem/DCS/Blueprints/Components/Inventory/BP_InventoryComponent.AddItem` _asbp_inventory_component _itemalrecoger (`self.CantidadItem`))
      (bind _asbp_equipment_component (cast `/Game/DynamicCombatSystem/DCS/Blueprints/Components/Inventory/BP_EquipmentComponent` (`self.GetComponentByClass` Caller "/Game/DynamicCombatSystem/DCS/Blueprints/Components/Inventory/BP_EquipmentComponent.BP_EquipmentComponent_C"))
        (:`then`
          (bind _itemfound (`/Game/DynamicCombatSystem/DCS/Blueprints/Components/Inventory/BP_InventoryComponent.FindItem` _asbp_inventory_component _itemalrecoger))
          (if _itemfound
            (`/Game/DynamicCombatSystem/DCS/Blueprints/Components/Inventory/BP_EquipmentComponent.UpdateItemInSlot` _asbp_equipment_component (`.Type_57_2423B0F4494306D370CCB1A1CAF5F77A` (break `/Game/DynamicCombatSystem/DCS/Blueprints/Components/Inventory/F_Item` (`/Game/DynamicCombatSystem/DCS/Blueprints/Items/ObjectItems/BP_DA_Item_Base.Item` _itemalrecoger))) 0 0 (`/Game/DynamicCombatSystem/DCS/Blueprints/Components/Inventory/BP_InventoryComponent.GetItemAtIndex` _asbp_inventory_component (- (`KismetArrayLibrary.Array_Length` (`/Game/DynamicCombatSystem/DCS/Blueprints/Components/Inventory/BP_InventoryComponent.Inventory` _asbp_inventory_component)) 1)) "NewEnumerator1")
            (`self.K2_DestroyActor`)
            (else
              (`self.K2_DestroyActor`))))
        (:`CastFailed`
          (`self.K2_DestroyActor`))))
    (:`Is Not Valid`
      (`self.K2_DestroyActor`))))

(event `self.ReceiveTick`
  (params (DeltaSeconds :type "Float (single-precision)"))
  (`parent.ReceiveTick` DeltaSeconds)
  (`self.PulsarLuz`))

(fn `Caer`
  (bind _mesh (`self.Mesh`))
  (set `self.Posado` false)
  (`PrimitiveComponent.SetCollisionEnabled` (`self.Zona`) "NoCollision")
  (`PrimitiveComponent.SetCollisionProfileName` _mesh "PhysicsActor" true)
  (`PrimitiveComponent.SetCollisionResponseToChannel` _mesh "ECC_Pawn" "ECR_Ignore")
  (`PrimitiveComponent.SetCollisionResponseToChannel` _mesh "ECC_PhysicsBody" "ECR_Ignore")
  (`PrimitiveComponent.SetUseCCD` _mesh true "None")
  (`PrimitiveComponent.SetSimulatePhysics` _mesh true)
  (`KismetSystemLibrary.K2_SetTimer` self "ComprobarPosado" 0.2 true false)
  (`KismetSystemLibrary.K2_SetTimer` self "Posar" 6.0))

(fn `CanjearTemporal`
  (params (Quien :type "Actor Object Reference") (Nueva :type "/Game/DynamicCombatSystem/DCS/Blueprints/Items/ObjectItems/BP_DA_Item_Base Object Reference"))
  (bind _asbp_da_player_character (cast `/Game/DarkAngels/Blueprints/Characters/BP_DA_PlayerCharacter` Quien))
  (`/Game/DarkAngels/Blueprints/Characters/BP_DA_PlayerCharacter.SustituirArmaTemporal` _asbp_da_player_character Nueva)
  (`/Game/DarkAngels/Blueprints/Characters/BP_DA_PlayerCharacter.RegistrarOrigenArma` _asbp_da_player_character (`self.EnemigoOrigen`))
  (`KismetSystemLibrary.K2_SetTimer` _asbp_da_player_character "CorromperArmaTemporal" 0.6))

(fn `ComprobarPosado`
  (bind _returnvalue (`PrimitiveComponent.GetPhysicsLinearVelocity` (`self.Mesh`) "None"))
  (if (< (`KismetMathLibrary.VSize` _returnvalue) 12.0)
    (`self.Posar`)))

(fn `MontarPilar`
  (bind _returnvalue (`|AddComponentByClass` :`self` self :`Class` "/Script/Engine.StaticMeshComponent"))
  (bind _asstatic_mesh_component (cast `StaticMeshComponent` _returnvalue))
  (set `self.Pilar` _asstatic_mesh_component)
  (`StaticMeshComponent.SetStaticMesh` (`self.Pilar`) "/Engine/BasicShapes/Cone.Cone")
  (`PrimitiveComponent.SetMaterial` (`self.Pilar`) 0 "/Game/DarkAngels/Materials/MI_DA_PilarArma.MI_DA_PilarArma")
  (`PrimitiveComponent.SetCollisionEnabled` (`self.Pilar`) "NoCollision")
  (`LightComponent.SetLightColor` (`self.Luz`) (make `LinearColor` 0.3 0.62 1.0 1.0) true)
  (`LocalLightComponent.SetAttenuationRadius` (`self.Luz`) 900.0)
  (`GameplayStatics.PlaySoundAtLocation` "/Game/DarkAngels/Audio/SC_DA_ArmaDisponible.SC_DA_ArmaDisponible" (`self.K2_GetActorLocation` self) (struct) 1.0 1.0 0.0 null null null null))

(fn `OcultarCartel`
  (params (Quien :type "Actor Object Reference"))
  (bind _asbp_combat_character (cast `/Game/DynamicCombatSystem/DCS/Blueprints/BP_CombatCharacter` Quien))
  (bind _ingamewidget (`/Game/DynamicCombatSystem/DCS/Blueprints/BP_CombatCharacter.InGameWidget` _asbp_combat_character))
  (`/Engine/EditorBlueprintResources/StandardMacros.IsValid` _ingamewidget
    (:`Is Valid`
      (bind _wb_interactionmessage (`/Game/DynamicCombatSystem/DCS/Widgets/WB_InGame.WB_InteractionMessage` _ingamewidget))
      (`/Engine/EditorBlueprintResources/StandardMacros.IsValid` _wb_interactionmessage
        (:`Is Valid`
          (`/Game/DynamicCombatSystem/DCS/Widgets/Interaction/WB_InteractionMessage.UpdateWidget` _wb_interactionmessage "None"))))))

(fn `Posar`
  (bind _mesh (`self.Mesh`))
  (bind _returnvalue (`SceneComponent.K2_GetComponentLocation` _mesh))
  (if (not (`self.Posado`))
    (set `self.Posado` true)
    (`KismetSystemLibrary.K2_ClearTimer` self "ComprobarPosado")
    (`PrimitiveComponent.SetSimulatePhysics` _mesh false)
    (`PrimitiveComponent.SetCollisionProfileName` _mesh "NoCollision" true)
    (bind (_outhit _returnvalue_2) (`KismetSystemLibrary.LineTraceSingle` (+ _returnvalue (`KismetMathLibrary.MakeVector` 0.0 0.0 200.0)) (- _returnvalue (`KismetMathLibrary.MakeVector` 0.0 0.0 2000.0)) "TraceTypeQuery1"))
    (`self.K2_SetActorLocationAndRotation` self (select `bool` _returnvalue_2 :`false` _returnvalue :`true` (`.Location` (`GameplayStatics.BreakHitResult` _outhit))) (`SceneComponent.K2_GetComponentRotation` _mesh) false true)
    (`SceneComponent.K2_SetRelativeLocation` _mesh (`KismetMathLibrary.MakeVector` 0.0) false false)
    (`SceneComponent.K2_SetRelativeRotation` _mesh (`KismetMathLibrary.MakeRotator` 0.0) false false)
    (`PrimitiveComponent.SetCollisionEnabled` (`self.Zona`) "QueryOnly")))

(fn `PulsarLuz`
  (bind _pilar (`self.Pilar`))
  (bind _alturapilar (`self.AlturaPilar`))
  (bind _mesh (`self.Mesh`))
  (bind (_min _max) (`StaticMeshComponent.GetLocalBounds` _mesh))
  (bind _returnvalue (+ 0.78 (* 0.22 (`KismetMathLibrary.Sin` (* (`KismetSystemLibrary.GetGameTimeInSeconds`) 2.6)))))
  (bind _returnvalue_2 (`KismetMathLibrary.TransformLocation` (`SceneComponent.K2_GetComponentToWorld` _mesh) (`KismetMathLibrary.MakeVector` (/ (+ (.x _min) (.x _max)) 2.0) (/ (+ (.y _min) (.y _max)) 2.0) (/ (+ (.z _min) (.z _max)) 2.0))))
  (bind _returnvalue_3 (* (`KismetMathLibrary.FMax` (/ (`KismetMathLibrary.FMax` (`KismetMathLibrary.FMax` (- (.x _max) (.x _min)) (- (.y _max) (.y _min))) (- (.z _max) (.z _min))) 100.0) 0.75) (+ 0.85 (* 0.15 _returnvalue))))
  (`LightComponent.SetIntensity` (`self.Luz`) (* 6000.0 _returnvalue))
  (`/Engine/EditorBlueprintResources/StandardMacros.IsValid` _pilar
    (:`Is Valid`
      (`SceneComponent.K2_SetWorldRotation` _pilar (`KismetMathLibrary.MakeRotator` 0.0) false false)
      (`SceneComponent.K2_SetWorldLocation` _pilar (`KismetMathLibrary.MakeVector` (.x _returnvalue_2) (.y _returnvalue_2) (+ (.z (`self.K2_GetActorLocation` self)) (* _alturapilar 0.5))) false false)
      (`SceneComponent.SetRelativeScale3D` _pilar (`KismetMathLibrary.MakeVector` _returnvalue_3 _returnvalue_3 (* _alturapilar 0.01))))))

(fn `RegistrarOrigen`
  (params (Nombre :type String))
  (set `self.EnemigoOrigen` Nombre))

(fn `SetItemDrop`
  (params (NewItem :type "/Game/DynamicCombatSystem/DCS/Blueprints/Items/ObjectItems/BP_DA_Item_Base Object Reference"))
  (set `self.ItemAlRecoger` NewItem))

(fn `UserConstructionScript`
  (`parent.UserConstructionScript`))

(fn `ZZProbePilar`)