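; Ground marker actor for an arrow rain attack, showing the target area and spawning the falling arrows over it.
; On BeginPlay it builds a tinted, collisionless plane scaled to Radio, spawns NumFlechas BP_DA_FlechaLluvia actors at random offsets overhead, plays a sound and expires after a short lifespan.
; Lanzar repeats this logic with count and radius parameters, a different material, fixed spawn height and no sound.
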(event `self.ReceiveBeginPlay`
  (bind _returnvalue (`|AddComponentByClass` :`self` self :`Class` "/Script/Engine.StaticMeshComponent"))
  (bind _asstatic_mesh_component (cast `StaticMeshComponent` _returnvalue))
  (`StaticMeshComponent.SetStaticMesh` _asstatic_mesh_component "/Engine/BasicShapes/Plane.Plane")
  (bind _returnvalue_2 (`PrimitiveComponent.CreateDynamicMaterialInstance` _asstatic_mesh_component 0 "/Game/DarkAngels/Materials/M_DA_Aura.M_DA_Aura" "None"))
  (`MaterialInstanceDynamic.SetVectorParameterValue` _returnvalue_2 "Color" (make `LinearColor` 1.0 0.92 0.7 1.0))
  (`PrimitiveComponent.SetCollisionEnabled` _asstatic_mesh_component "NoCollision")
  (`SceneComponent.K2_SetRelativeLocation` _asstatic_mesh_component (`KismetMathLibrary.MakeVector` 0.0 0.0 3.0) false false)
  (`SceneComponent.SetRelativeScale3D` _asstatic_mesh_component (`KismetMathLibrary.MakeVector` (* (`self.Radio`) 0.02) (* (`self.Radio`) 0.02) 1.0))
  (for _ (range (+ (- (`self.NumFlechas`) 1) 1))
    (`|SpawnActorFromClass` "/Game/DarkAngels/Blueprints/Combat/BP_DA_FlechaLluvia.BP_DA_FlechaLluvia_C" (`KismetMathLibrary.MakeTransform` (`KismetMathLibrary.MakeVector` (+ (.x (`self.K2_GetActorLocation` self)) (`KismetMathLibrary.RandomFloatInRange` (- 0.0 (* (`self.Radio`) 0.85)) (* (`self.Radio`) 0.85))) (+ (.y (`self.K2_GetActorLocation` self)) (`KismetMathLibrary.RandomFloatInRange` (- 0.0 (* (`self.Radio`) 0.85)) (* (`self.Radio`) 0.85))) (+ (.z (`self.K2_GetActorLocation` self)) (+ (`self.AlturaSalida`) (`KismetMathLibrary.RandomFloatInRange` -400.0 400.0))))) "AlwaysSpawn" "MultiplyWithRoot" self null))
  (`self.SetLifeSpan` self 4.0)
  (`GameplayStatics.PlaySound2D` "/Game/DarkAngels/Audio/SFX/rain_pulse.rain_pulse" 1.0 1.0 0.0 null null))

(fn `Lanzar`
  (params (Cuantas :type Integer) (Radio :type "Float (double-precision)"))
  (bind _returnvalue (`|AddComponentByClass` :`self` self :`Class` "/Script/Engine.StaticMeshComponent"))
  (bind _asstatic_mesh_component (cast `StaticMeshComponent` _returnvalue))
  (`StaticMeshComponent.SetStaticMesh` _asstatic_mesh_component "/Engine/BasicShapes/Plane.Plane")
  (bind _returnvalue_2 (`PrimitiveComponent.CreateDynamicMaterialInstance` _asstatic_mesh_component 0 "/Game/DarkAngels/Materials/MI_DA_MarcaLluvia.MI_DA_MarcaLluvia" "None"))
  (`MaterialInstanceDynamic.SetVectorParameterValue` _returnvalue_2 "Color" (make `LinearColor` 1.0 0.92 0.7 1.0))
  (`PrimitiveComponent.SetCollisionEnabled` _asstatic_mesh_component "NoCollision")
  (`SceneComponent.K2_SetRelativeLocation` _asstatic_mesh_component (`KismetMathLibrary.MakeVector` 0.0 0.0 3.0) false false)
  (`SceneComponent.SetRelativeScale3D` _asstatic_mesh_component (`KismetMathLibrary.MakeVector` (* Radio 0.02) (* Radio 0.02) 1.0))
  (for _ (range (+ (- Cuantas 1) 1))
    (`|SpawnActorFromClass` "/Game/DarkAngels/Blueprints/Combat/BP_DA_FlechaLluvia.BP_DA_FlechaLluvia_C" (`KismetMathLibrary.MakeTransform` (`KismetMathLibrary.MakeVector` (+ (.x (`self.K2_GetActorLocation` self)) (`KismetMathLibrary.RandomFloatInRange` (- 0.0 (* Radio 0.85)) (* Radio 0.85))) (+ (.y (`self.K2_GetActorLocation` self)) (`KismetMathLibrary.RandomFloatInRange` (- 0.0 (* Radio 0.85)) (* Radio 0.85))) (+ (.z (`self.K2_GetActorLocation` self)) (+ 3000.0 (`KismetMathLibrary.RandomFloatInRange` -400.0 400.0))))) "AlwaysSpawn" "MultiplyWithRoot" self null))
  (`self.SetLifeSpan` self 4.0))

(fn `UserConstructionScript`)