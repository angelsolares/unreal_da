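; BP_DA_FlechaLluvia is a cosmetic falling arrow, named as part of an arrow rain in Dark Angels combat.
; BeginPlay adds a downward-pitched, collision-free elven arrow mesh, takes the owner's Z as ground height and sets a short lifespan.
; Tick lowers it at a constant fall speed without sweeps, then snaps it to that height and flags it as stuck (Clavada).
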(event `self.ReceiveBeginPlay`
  (bind _returnvalue (`|AddComponentByClass` :`self` self :`Class` "/Script/Engine.StaticMeshComponent"))
  (bind _asstatic_mesh_component (cast `StaticMeshComponent` _returnvalue))
  (`StaticMeshComponent.SetStaticMesh` _asstatic_mesh_component "/Game/DynamicCombatSystem/DCS/Meshes/SM_ElvenArrow.SM_ElvenArrow")
  (`PrimitiveComponent.SetCollisionEnabled` _asstatic_mesh_component "NoCollision")
  (`SceneComponent.K2_SetRelativeRotation` _asstatic_mesh_component (`KismetMathLibrary.MakeRotator` 0.0 -90.0) false false)
  (`SceneComponent.SetRelativeScale3D` _asstatic_mesh_component (`KismetMathLibrary.MakeVector` 1.4 1.4 1.4))
  (set `self.ZSuelo` (.z (`self.K2_GetActorLocation` (`self.GetOwner`))))
  (`self.SetLifeSpan` self 5.0))

(event `self.ReceiveTick`
  (params (DeltaSeconds :type "Float (single-precision)"))
  (if (not (`self.Clavada`))
    (if (<= (- (.z (`self.K2_GetActorLocation` self)) (* (`self.VelocidadCaida`) DeltaSeconds)) (`self.ZSuelo`))
      (`self.K2_SetActorLocation` self (`KismetMathLibrary.MakeVector` (.x (`self.K2_GetActorLocation` self)) (.y (`self.K2_GetActorLocation` self)) (`self.ZSuelo`)) false false)
      (set `self.Clavada` true)
      (else
        (`self.K2_SetActorLocation` self (`KismetMathLibrary.MakeVector` (.x (`self.K2_GetActorLocation` self)) (.y (`self.K2_GetActorLocation` self)) (- (.z (`self.K2_GetActorLocation` self)) (* (`self.VelocidadCaida`) DeltaSeconds))) false false)))))

(fn `UserConstructionScript`)