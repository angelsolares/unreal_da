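; Animation notify that triggers banner planting (PlantarEstandarte) on the Dark Angels player character.
; On Received_Notify it casts the mesh owner to BP_DA_PlayerCharacter, calls that function and returns true if the character is valid.
; The graph also holds disconnected leftovers that never run: a parent call, a scaled finisher camera shake and a temporary weapon throw (ArrojarArmaTemporal).
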(fn `Received_Notify`
  (params (MeshComp :type "SkeletalMeshComponent Object Reference") (Animation :type "AnimSequenceBase Object Reference") (EventReference :type "AnimNotifyEventReference Structure (by ref)"))
  (returns (ReturnValue :type Boolean))
  (bind _asbp_da_player_character (cast `/Game/DarkAngels/Blueprints/Characters/BP_DA_PlayerCharacter` (`ActorComponent.GetOwner` MeshComp)))
  (`/Engine/EditorBlueprintResources/StandardMacros.IsValid` _asbp_da_player_character
    (:`Is Valid`
      (`/Game/DarkAngels/Blueprints/Characters/BP_DA_PlayerCharacter.PlantarEstandarte` _asbp_da_player_character)
      (return true))
    (:`Is Not Valid`
      (return false))))