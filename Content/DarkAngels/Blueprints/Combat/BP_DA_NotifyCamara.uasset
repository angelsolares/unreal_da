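; Animation notify that snaps the player's camera to a framed shot of the animated pawn, apparently for combat.
; It acts only when the owner is a pawn with a player controller whose view target is a CameraActor.
; The camera is placed from owner-relative forward, side and height offsets, turned toward an offset aim point on the owner's axes, and given a new FOV, without blending.
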(fn `Received_Notify`
  (params (MeshComp :type "SkeletalMeshComponent Object Reference") (Animation :type "AnimSequenceBase Object Reference") (EventReference :type "AnimNotifyEventReference Structure (by ref)"))
  (returns (ReturnValue :type Boolean))
  (bind _returnvalue (`ActorComponent.GetOwner` MeshComp))
  (bind _returnvalue_2 (+ (`Actor.K2_GetActorLocation` _returnvalue) (* (`Actor.GetActorForwardVector` _returnvalue) (`self.Desfase`))))
  (bind _returnvalue_3 (+ (+ (+ _returnvalue_2 (* (`Actor.GetActorRightVector` _returnvalue) (`self.Lado`))) (* (`Actor.GetActorForwardVector` _returnvalue) (`self.Frente`))) (* (`Actor.GetActorUpVector` _returnvalue) (`self.Alto`))))
  (bind _aspawn (cast `Pawn` _returnvalue))
  (bind _asplayer_controller (cast `PlayerController` (`Pawn.GetController` _aspawn)))
  (bind _ascamera_actor (cast `CameraActor` (`Controller.GetViewTarget` _asplayer_controller)))
  (`Actor.K2_SetActorLocationAndRotation` _ascamera_actor _returnvalue_3 (`KismetMathLibrary.FindLookAtRotation` _returnvalue_3 (+ _returnvalue_2 (* (`Actor.GetActorUpVector` _returnvalue) (`self.Mira`)))) false false)
  (`CameraComponent.SetFieldOfView` (`CameraActor.CameraComponent` _ascamera_actor) (`self.FOV`))
  (return false))