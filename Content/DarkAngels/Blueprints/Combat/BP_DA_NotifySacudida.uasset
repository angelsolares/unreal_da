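; Animation notify that plays the finisher camera shake for the player whose pawn owns the animated mesh.
; On receipt it casts the mesh owner to a Pawn and its controller to a PlayerController, so AI and non-pawn owners get no shake.
; It starts CS_DA_Finisher through ClientStartCameraShake, scaled by the Escala variable, falling back to full scale when that is not positive.
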(fn `Received_Notify`
  (params (MeshComp :type "SkeletalMeshComponent Object Reference") (Animation :type "AnimSequenceBase Object Reference") (EventReference :type "AnimNotifyEventReference Structure (by ref)"))
  (returns (ReturnValue :type Boolean))
  (bind _aspawn (cast `Pawn` (`ActorComponent.GetOwner` MeshComp)))
  (bind _asplayer_controller (cast `PlayerController` (`Pawn.GetController` _aspawn)))
  (`PlayerController.ClientStartCameraShake` :`self` _asplayer_controller :`Shake` "/Game/DarkAngels/FX/CS_DA_Finisher.CS_DA_Finisher_C" :`Scale` (select `bool` (> (`self.Escala`) 0.0) :`false` 1.0 :`true` (`self.Escala`)))
  (return false))