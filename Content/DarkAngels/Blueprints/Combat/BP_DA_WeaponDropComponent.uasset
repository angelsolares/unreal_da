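; Actor component that drops the owner's equipped weapons as world pickups when it dies.
; A looping timer polls the owner's alive state, then once takes the off-hand and main-hand items from the equipment component, with a fallback main-hand slot type.
; Each drop spawns a BP_DA_DroppedWeapon copying the displayed mesh and transform, assigns the item and lifespan, hides the original and calls Caer.
; An unused ground-trace placement variant remains unwired.
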(event `self.ReceiveBeginPlay`
  (`KismetSystemLibrary.K2_SetTimer` self "CheckOwnerDeath" 0.5 true))

(event `CheckOwnerDeath`
  (bind _returnvalue (`self.GetOwner`))
  (bind _result (message `/Game/DynamicCombatSystem/DCS/Blueprints/Interfaces/I_CanBeAttacked.IsAlive` _returnvalue))
  (if (and (not _result) (not (`self.Dropped`)))
    (set `self.Dropped` true)
    (bind _asbp_equipment_component (cast `/Game/DynamicCombatSystem/DCS/Blueprints/Components/Inventory/BP_EquipmentComponent` (`Actor.GetComponentByClass` _returnvalue "/Game/DynamicCombatSystem/DCS/Blueprints/Components/Inventory/BP_EquipmentComponent.BP_EquipmentComponent_C")))
    (if (`self.DropOffHandWeapon`)
      (bind _item (`/Game/DynamicCombatSystem/DCS/Blueprints/Components/Inventory/BP_EquipmentComponent.GetActiveItem` _asbp_equipment_component "NewEnumerator6" 0))
      (bind _offhanddisplayeditem (message `/Game/DynamicCombatSystem/DCS/Blueprints/Interfaces/I_Character_UsesDisplayedItems.GetOffhandDisplayedItem` _returnvalue))
      (`self.DropOne` self _offhanddisplayeditem (`.Item_19_91F4466B44F35A055E90E1A872CB8B97` (break `/Game/DynamicCombatSystem/DCS/Blueprints/Components/Inventory/F_StoredItem` _item))))
    (if (`self.DropMainHandWeapon`)
      (bind _item_2 (`/Game/DynamicCombatSystem/DCS/Blueprints/Components/Inventory/BP_EquipmentComponent.GetActiveItem` _asbp_equipment_component "NewEnumerator18" 0))
      (bind _mainhanddisplayeditem (message `/Game/DynamicCombatSystem/DCS/Blueprints/Interfaces/I_Character_UsesDisplayedItems.GetMainHandDisplayedItem` _returnvalue))
      (bind (_id _item_3) (break `/Game/DynamicCombatSystem/DCS/Blueprints/Components/Inventory/F_StoredItem` _item_2))
      (`/Engine/EditorBlueprintResources/StandardMacros.IsValid` _item_3
        (:`Is Valid`
          (`self.DropOne` self _mainhanddisplayeditem _item_3))
        (:`Is Not Valid`
          (bind _item_4 (`/Game/DynamicCombatSystem/DCS/Blueprints/Components/Inventory/BP_EquipmentComponent.GetActiveItem` _asbp_equipment_component "NewEnumerator19" 0))
          (bind (_id_2 _item_5) (break `/Game/DynamicCombatSystem/DCS/Blueprints/Components/Inventory/F_StoredItem` _item_4))
          (`/Engine/EditorBlueprintResources/StandardMacros.IsValid` _item_5
            (:`Is Valid`
              (`self.DropOne` self _mainhanddisplayeditem _item_5))))))))

(fn `DropOne`
  (params (Item :type "Actor Object Reference") (WeaponItem :type "/Game/DynamicCombatSystem/DCS/Blueprints/Items/ObjectItems/BP_DA_Item_Base Object Reference"))
  (`/Engine/EditorBlueprintResources/StandardMacros.IsValid` Item
    (:`Is Valid`
      (bind _asstatic_mesh_component (cast `StaticMeshComponent` (`Actor.GetComponentByClass` Item "/Script/Engine.StaticMeshComponent")))
      (bind _returnvalue (`|SpawnActorFromClass` "/Game/DarkAngels/Blueprints/Combat/BP_DA_DroppedWeapon.BP_DA_DroppedWeapon_C" (`KismetMathLibrary.MakeTransform` (`SceneComponent.K2_GetComponentLocation` _asstatic_mesh_component) (`SceneComponent.K2_GetComponentRotation` _asstatic_mesh_component)) "AlwaysSpawn" "MultiplyWithRoot" null null))
      (bind _asbp_da_dropped_weapon (cast `/Game/DarkAngels/Blueprints/Combat/BP_DA_DroppedWeapon` _returnvalue))
      (`StaticMeshComponent.SetStaticMesh` (`/Game/DarkAngels/Blueprints/Combat/BP_DA_DroppedWeapon.Mesh` _asbp_da_dropped_weapon) (`StaticMeshComponent.StaticMesh` _asstatic_mesh_component))
      (`/Game/DarkAngels/Blueprints/Combat/BP_DA_DroppedWeapon.SetItemDrop` _asbp_da_dropped_weapon WeaponItem)
      (`Actor.SetLifeSpan` _asbp_da_dropped_weapon (`self.DropLifeSpan`))
      (`Actor.SetActorEnableCollision` Item false)
      (`Actor.SetActorHiddenInGame` Item true)
      (`/Game/DarkAngels/Blueprints/Combat/BP_DA_DroppedWeapon.Caer` _asbp_da_dropped_weapon))))