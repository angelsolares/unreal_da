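; Planted shield actor that acts as a wall, bouncing enemy projectiles back within a fixed radius.
; A looping timer started on BeginPlay runs Barrer, which polls all BP_BaseMovingProjectile actors for proximity and hostile owners instead of using collision.
; Each match prints a debug message, is re-owned to the shield's owner and has its velocity set backwards along local X at the same speed.
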(event `self.ReceiveBeginPlay`
  (`KismetSystemLibrary.K2_SetTimer` self "Barrer" 0.05 true))

(fn `Barrer`
  (bind _outactors (`GameplayStatics.GetAllActorsOfClass` "/Game/DynamicCombatSystem/DCS/Blueprints/Projectiles/BP_BaseMovingProjectile.BP_BaseMovingProjectile_C"))
  (for _array_element _outactors
    (if (and (< (`KismetMathLibrary.VSize` (- (`self.K2_GetActorLocation` _array_element) (`self.K2_GetActorLocation` self))) 420.0) (`/Game/DynamicCombatSystem/DCS/Blueprints/BP_DCSLibrary.IsEnemy` (`self.GetOwner` self) (`self.GetOwner` _array_element)))
      (`KismetSystemLibrary.PrintString` "MURO REBOTA" false true (struct :`G` 0.66 :`B` 1.0 :`A` 1.0) 0.0)
      (bind _asprojectile_movement_component (cast `ProjectileMovementComponent` (`self.GetComponentByClass` _array_element "/Script/Engine.ProjectileMovementComponent")))
      (`self.SetOwner` _array_element (`self.GetOwner` self))
      (`ProjectileMovementComponent.SetVelocityInLocalSpace` _asprojectile_movement_component (`KismetMathLibrary.MakeVector` (- 0.0 (`KismetMathLibrary.VSize` (`self.GetVelocity` _array_element))))))))

(fn `UserConstructionScript`)