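; Stages a one-shot angel descent for an arena wave, lifting enemies into the air so they drop in.
; A looping timer runs the sequence once armed by Arrancar or the nearby BP_DA_Arena's wave count.
; Sembrar spawns one Vigilante or gathers tagged actors in radius; after a delay, Alzar raises them, plays flapping and stops AI logic.
; Aterrizar restores Animation Blueprints and restarts AI once all have landed.
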(event `self.ReceiveBeginPlay`
  (`KismetSystemLibrary.K2_SetTimer` self "Vigilar" 0.1 true))

(fn `Alzar`
  (for _array_element (`self.Cayendo`)
    (`self.K2_SetActorLocation` _array_element (+ (`self.K2_GetActorLocation` _array_element) (`KismetMathLibrary.MakeVector` 0.0 0.0 (`self.Altura`))) false false)
    (for _array_element_2 (`self.K2_GetComponentsByClass` _array_element "/Script/Engine.SkeletalMeshComponent")
      (`SkeletalMeshComponent.SetAnimationMode` _array_element_2 "AnimationSingleNode" true)
      (`SkeletalMeshComponent.PlayAnimation` _array_element_2 "/Game/GiantBossProject/Demo/Characters/Mannequins/Animations/Manny/MM_Fall_Loop.MM_Fall_Loop" true)
      (`SkeletalMeshComponent.PlayAnimation` _array_element_2 "/Game/Angel_wings_pack/Animations/5/Animations/AS__AS_W5_flapping.AS__AS_W5_flapping" true))
    (`/Engine/EditorBlueprintResources/StandardMacros.IsValid` (`AIBlueprintHelperLibrary.GetAIController` _array_element)
      (:`Is Valid`
        (`BrainComponent.StopLogic` (`AIController.BrainComponent` (`AIBlueprintHelperLibrary.GetAIController` _array_element)) "descenso")))))

(fn `Arrancar`
  (set `self.Armado` true))

(fn `Aterrizar`
  (set `self.AlgunoVolando` false)
  (for _array_element (`self.Cayendo`)
    (if (or (`NavMovementInterface.IsFalling` (`self.GetComponentByClass` _array_element "/Script/Engine.CharacterMovementComponent")) (> (.z (`self.K2_GetActorLocation` _array_element)) (+ (.z (`self.K2_GetActorLocation`)) 300.0)))
      (set `self.AlgunoVolando` true)))
  (if (and (not (`self.AlgunoVolando`)) (> (`KismetArrayLibrary.Array_Length` (`self.Cayendo`)) 0))
    (for _array_element_2 (`self.Cayendo`)
      (for _array_element_3 (`self.K2_GetComponentsByClass` _array_element_2 "/Script/Engine.SkeletalMeshComponent")
        (`SkeletalMeshComponent.SetAnimationMode` _array_element_3 "AnimationBlueprint" true))
      (`/Engine/EditorBlueprintResources/StandardMacros.IsValid` (`AIBlueprintHelperLibrary.GetAIController` _array_element_2)
        (:`Is Valid`
          (`BrainComponent.RestartLogic` (`AIController.BrainComponent` (`AIBlueprintHelperLibrary.GetAIController` _array_element_2))))))
    (`KismetArrayLibrary.Array_Clear` (`self.Cayendo`))
    (`KismetSystemLibrary.PrintString` "DESCENSO: han tocado suelo")))

(fn `Sembrar`
  (if (`self.SoloSpawn`)
    (bind _returnvalue (`|SpawnActorFromClass` "/Game/DarkAngels/Blueprints/Enemies/BP_DA_Vigilante.BP_DA_Vigilante_C" (`KismetMathLibrary.MakeTransform` (`self.K2_GetActorLocation`)) "AdjustIfPossibleButAlwaysSpawn" "MultiplyWithRoot" self null))
    (`KismetArrayLibrary.Array_Add` (`self.Cayendo`) _returnvalue)
    (else
      (bind _outactors (`GameplayStatics.GetAllActorsWithTag` (`self.TagOleada`)))
      (for _array_element _outactors
        (if (< (`KismetMathLibrary.Vector_Distance` (`self.K2_GetActorLocation` _array_element) (`self.K2_GetActorLocation`)) (`self.Radio`))
          (`KismetArrayLibrary.Array_Add` (`self.Cayendo`) _array_element))))))

(fn `UserConstructionScript`)

(fn `Vigilar`
  (if (and (not (`self.Hecho`)) (`self.Armado`))
    (set `self.Hecho` true)
    (`self.Sembrar`)
    (set `self.PendienteAlzar` true)
    (set `self.Espera` 0.6)
    (`KismetSystemLibrary.PrintString` "DESCENSO: los angeles se preparan"))
  (if (> (`self.Espera`) 0.0)
    (set `self.Espera` (- (`self.Espera`) 0.1))
    (elif (`self.PendienteAlzar`)
      (set `self.PendienteAlzar` false)
      (set `self.Espera` 0.6)
      (`self.Alzar`)
      (`KismetSystemLibrary.PrintString` "DESCENSO: los angeles bajan")
      (else
        (`self.Aterrizar`))))
  (if (not (`self.SoloSpawn`))
    (`/Engine/EditorBlueprintResources/StandardMacros.IsValid` (`self.Arena`)
      (:`Is Valid`
        (bind _asbp_da_arena (cast `/Game/DarkAngels/Blueprints/Combat/BP_DA_Arena` (`self.Arena`)))
        (if (>= (`/Game/DarkAngels/Blueprints/Combat/BP_DA_Arena.OleadaActual` _asbp_da_arena) (`self.OleadaDisparo`))
          (set `self.Armado` true)))
      (:`Is Not Valid`
        (bind _outactors (`GameplayStatics.GetAllActorsOfClass` "/Game/DarkAngels/Blueprints/Combat/BP_DA_Arena.BP_DA_Arena_C"))
        (for _array_element _outactors
          (if (< (`KismetMathLibrary.Vector_Distance` (`self.K2_GetActorLocation` _array_element) (`self.K2_GetActorLocation`)) (`self.Radio`))
            (set `self.Arena` _array_element)))))))