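; Aura component that adds a Stat.Damage modifier, positive or negative, to living BP_BaseAI actors near its owner, excluding the owner.
; Unless SiempreActiva, it waits for player proximity plus a delay, then spawns a ground ring and light colored by bonus sign.
; A one-second timer removes and reapplies modifiers while the owner lives or SiempreActiva, skipping spots the player's BP_DA_Vetas reports silenced.
; EndPlay clears timers and modifiers.
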(event `self.ReceiveBeginPlay`
  (`self.ArrancarAura`))

(event `self.ReceiveEndPlay`
  (params (EndPlayReason :type "EEndPlayReason Enum" :default "Destroyed"))
  (`self.LimpiarArranque`)
  (`KismetSystemLibrary.K2_ClearTimer` self "RevisarAura")
  (`self.QuitarATodos`))

(fn `ActivarAura`
  (`self.MontarVisual`)
  (`KismetSystemLibrary.K2_SetTimer` self "RevisarAura" 1.0 true))

(fn `ArrancarAura`
  (if (`self.SiempreActiva`)
    (`self.ActivarAura`)
    (else
      (`KismetSystemLibrary.K2_SetTimer` self "VigilarArranque" 0.5 true))))

(fn `LimpiarArranque`
  (`KismetSystemLibrary.K2_ClearTimer` self "VigilarArranque")
  (`KismetSystemLibrary.K2_ClearTimer` self "ActivarAura"))

(fn `MontarVisual`
  (bind _anillo (`self.Anillo`))
  (bind _luzaura (`self.LuzAura`))
  (bind _radioaura (`self.RadioAura`))
  (bind _returnvalue (`self.GetOwner` self))
  (bind _returnvalue_2 (`|AddComponentByClass` :`self` _returnvalue :`Class` "/Script/Engine.StaticMeshComponent"))
  (bind _asstatic_mesh_component (cast `StaticMeshComponent` _returnvalue_2))
  (set `self.Anillo` _asstatic_mesh_component)
  (`StaticMeshComponent.SetStaticMesh` _anillo "/Engine/BasicShapes/Plane.Plane")
  (bind _returnvalue_3 (`PrimitiveComponent.CreateDynamicMaterialInstance` _anillo 0 "/Game/DarkAngels/Materials/M_DA_Aura.M_DA_Aura" "None"))
  (`PrimitiveComponent.SetCollisionEnabled` _anillo "NoCollision")
  (`SceneComponent.K2_SetRelativeLocation` _anillo (`KismetMathLibrary.MakeVector` 0.0 0.0 -85.0) false false)
  (`SceneComponent.SetRelativeScale3D` _anillo (`KismetMathLibrary.MakeVector` (* _radioaura 0.02) (* _radioaura 0.02) 1.0))
  (bind _returnvalue_4 (`|AddComponentByClass` :`self` _returnvalue :`Class` "/Script/Engine.PointLightComponent"))
  (bind _aspoint_light_component (cast `PointLightComponent` _returnvalue_4))
  (set `self.LuzAura` _aspoint_light_component)
  (`LightComponent.SetIntensity` _luzaura 6000.0)
  (`LocalLightComponent.SetAttenuationRadius` _luzaura (* _radioaura 0.6))
  (`SceneComponent.K2_SetRelativeLocation` _luzaura (`KismetMathLibrary.MakeVector` 0.0 0.0 40.0) false false)
  (if (< (`self.Bonificacion`) 0.0)
    (`MaterialInstanceDynamic.SetVectorParameterValue` _returnvalue_3 "Color" (make `LinearColor` 0.22 0.45 1.0 1.0))
    (`LightComponent.SetLightColor` _luzaura (make `LinearColor` 0.22 0.45 1.0 1.0) true)
    (else
      (`MaterialInstanceDynamic.SetVectorParameterValue` _returnvalue_3 "Color" (make `LinearColor` 1.0 0.35 0.12 1.0))
      (`LightComponent.SetLightColor` _luzaura (make `LinearColor` 1.0 0.35 0.12 1.0) true))))

(fn `QuitarATodos`
  (for _array_element (`self.Afectados`)
    (bind _asbp_stats_manager_component (cast `/Game/DynamicCombatSystem/DCS/Blueprints/Components/StatsManager/BP_StatsManagerComponent` (`Actor.GetComponentByClass` _array_element "/Game/DynamicCombatSystem/DCS/Blueprints/Components/StatsManager/BP_StatsManagerComponent.BP_StatsManagerComponent_C")))
    (`/Engine/EditorBlueprintResources/StandardMacros.IsValid` _asbp_stats_manager_component
      (:`Is Valid`
        (`/Game/DynamicCombatSystem/DCS/Blueprints/Components/StatsManager/BP_StatsManagerComponent.RemoveModifier` _asbp_stats_manager_component (`BlueprintGameplayTagLibrary.MakeLiteralGameplayTag` (struct :`TagName` "Stat.Damage")) (`self.Bonificacion`)))))
  (`KismetArrayLibrary.Array_Clear` (`self.Afectados`)))

(fn `RevisarAura`
  (bind _returnvalue (`self.GetOwner` self))
  (bind _result (message `/Game/DynamicCombatSystem/DCS/Blueprints/Interfaces/I_CanBeAttacked.IsAlive` _returnvalue))
  (`self.QuitarATodos`)
  (bind _returnvalue_2 (or _result (`self.SiempreActiva`)))
  (`SceneComponent.SetVisibility` (`self.Anillo`) _returnvalue_2 true)
  (`SceneComponent.SetVisibility` (`self.LuzAura`) _returnvalue_2 true)
  (bind _asbp_da_vetas (cast `/Game/DarkAngels/Blueprints/Combat/BP_DA_Vetas` (`Actor.GetComponentByClass` (`GameplayStatics.GetPlayerPawn` 0) "/Game/DarkAngels/Blueprints/Combat/BP_DA_Vetas.BP_DA_Vetas_C")))
  (if _returnvalue_2
    (bind _outactors (`GameplayStatics.GetAllActorsOfClass` "/Game/DynamicCombatSystem/DCS/Blueprints/AI/BP_BaseAI.BP_BaseAI_C"))
    (for _array_element _outactors
      (bind _result_2 (message `/Game/DynamicCombatSystem/DCS/Blueprints/Interfaces/I_CanBeAttacked.IsAlive` _array_element))
      (bind _returnvalue_3 (`Actor.K2_GetActorLocation` _array_element))
      (if (and (and (< (`KismetMathLibrary.Vector_Distance` (`Actor.K2_GetActorLocation` _returnvalue) _returnvalue_3) (`self.RadioAura`)) _result_2) (!= _array_element _returnvalue))
        (`/Engine/EditorBlueprintResources/StandardMacros.IsValid` _asbp_da_vetas
          (:`Is Valid`
            (bind _valor (`/Game/DarkAngels/Blueprints/Combat/BP_DA_Vetas.EnSilencio` _asbp_da_vetas _returnvalue_3))
            (if (not _valor)
              (bind _asbp_stats_manager_component (cast `/Game/DynamicCombatSystem/DCS/Blueprints/Components/StatsManager/BP_StatsManagerComponent` (`Actor.GetComponentByClass` _array_element "/Game/DynamicCombatSystem/DCS/Blueprints/Components/StatsManager/BP_StatsManagerComponent.BP_StatsManagerComponent_C")))
              (`/Engine/EditorBlueprintResources/StandardMacros.IsValid` _asbp_stats_manager_component
                (:`Is Valid`
                  (`/Game/DynamicCombatSystem/DCS/Blueprints/Components/StatsManager/BP_StatsManagerComponent.AddModifier` _asbp_stats_manager_component (struct :`TagName` "Stat.Damage") (`self.Bonificacion`))
                  (`KismetArrayLibrary.Array_Add` (`self.Afectados`) _array_element)))))
          (:`Is Not Valid`
            (bind _asbp_stats_manager_component_2 (cast `/Game/DynamicCombatSystem/DCS/Blueprints/Components/StatsManager/BP_StatsManagerComponent` (`Actor.GetComponentByClass` _array_element "/Game/DynamicCombatSystem/DCS/Blueprints/Components/StatsManager/BP_StatsManagerComponent.BP_StatsManagerComponent_C")))
            (`/Engine/EditorBlueprintResources/StandardMacros.IsValid` _asbp_stats_manager_component_2
              (:`Is Valid`
                (`/Game/DynamicCombatSystem/DCS/Blueprints/Components/StatsManager/BP_StatsManagerComponent.AddModifier` _asbp_stats_manager_component_2 (struct :`TagName` "Stat.Damage") (`self.Bonificacion`))
                (`KismetArrayLibrary.Array_Add` (`self.Afectados`) _array_element)))))))))

(fn `VigilarArranque`
  (bind _returnvalue (`GameplayStatics.GetPlayerCharacter` 0))
  (`/Engine/EditorBlueprintResources/StandardMacros.IsValid` _returnvalue
    (:`Is Valid`
      (if (< (`KismetMathLibrary.Vector_Distance` (`Actor.K2_GetActorLocation` _returnvalue) (`Actor.K2_GetActorLocation` (`self.GetOwner` self))) (`self.RadioArranque`))
        (`KismetSystemLibrary.K2_ClearTimer` self "VigilarArranque")
        (`KismetSystemLibrary.K2_SetTimer` self "ActivarAura" (`self.RetrasoAura`))))))

(fn `ZZProbeAura`)