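; Wings actor for a Herald in DarkAngels, attached to a parent actor and shown flapping while that parent rises.
; Each Tick compares the parent's Z with the previous frame's; a gain above UmbralSubida, a per-frame threshold not scaled by delta time, counts as flying.
; On state changes it either unhides and loops the flap animation, or loops the folded animation and hides the actor.
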(event `self.ReceiveBeginPlay`
  (`SkeletalMeshComponent.PlayAnimation` (`self.Alas`) (`self.AnimPlegadas`) true)
  (`/Engine/EditorBlueprintResources/StandardMacros.IsValid` (`self.GetAttachParentActor`)
    (:`Is Valid`
      (set `self.ZAnterior` (.z (`self.K2_GetActorLocation` (`self.GetAttachParentActor`)))))))

(event `self.ReceiveTick`
  (params (DeltaSeconds :type "Float (single-precision)"))
  (`/Engine/EditorBlueprintResources/StandardMacros.IsValid` (`self.GetAttachParentActor`)
    (:`Is Valid`
      (set `self.Subiendo` (> (- (.z (`self.K2_GetActorLocation` (`self.GetAttachParentActor`))) (`self.ZAnterior`)) (`self.UmbralSubida`)))
      (set `self.ZAnterior` (.z (`self.K2_GetActorLocation` (`self.GetAttachParentActor`))))
      (if (!= (`self.Subiendo`) (`self.Volando`))
        (set `self.Volando` (`self.Subiendo`))
        (if (`self.Volando`)
          (`self.SetActorHiddenInGame` self false)
          (`SkeletalMeshComponent.PlayAnimation` (`self.Alas`) (`self.AnimAleteo`) true)
          (else
            (`SkeletalMeshComponent.PlayAnimation` (`self.Alas`) (`self.AnimPlegadas`) true)
            (`self.SetActorHiddenInGame` self true)))))))

(fn `UserConstructionScript`)