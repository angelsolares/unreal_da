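; BP_DA_AlasMuerte is a component that handles its owner's death sequence, ending in dissolve and destruction.
; After a one-second startup delay, Tick polls the owner's IsAliveMessage and fires only once when it reports dead.
; It switches all the owner's skeletal meshes to single-node animation, waits, then dissolves each through the owner's BP_DissolveComponent.
; The owner is destroyed after a further configurable delay, SegundosHastaBorrar.
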(event `self.ReceiveBeginPlay`
  (`KismetSystemLibrary.Delay` 1.0)
  (set `self.Listo` true))

(event `self.ReceiveTick`
  (params (DeltaSeconds :type "Float (single-precision)"))
  (bind _result (message `/Game/DynamicCombatSystem/DCS/Blueprints/Interfaces/I_CanBeAttacked.IsAlive` (`self.GetOwner`)))
  (if (and (`self.Listo`) (and (not (`self.Muerto`)) (not _result)))
    (set `self.Muerto` true)
    (for _array_element (`Actor.K2_GetComponentsByClass` (`self.GetOwner`) "/Script/Engine.SkeletalMeshComponent")
      (`SkeletalMeshComponent.SetAnimationMode` _array_element "AnimationSingleNode" true))
    (`KismetSystemLibrary.Delay` 3.0)
    (for _array_element_2 (`Actor.K2_GetComponentsByClass` (`self.GetOwner`) "/Script/Engine.SkeletalMeshComponent")
      (`/Game/DynamicCombatSystem/DCS/Blueprints/Components/Dissolve/BP_DissolveComponent.StartDissolve` (`Actor.GetComponentByClass` (`self.GetOwner`) "/Game/DynamicCombatSystem/DCS/Blueprints/Components/Dissolve/BP_DissolveComponent.BP_DissolveComponent_C") _array_element_2 false))
    (`KismetSystemLibrary.Delay` (`self.SegundosHastaBorrar`))
    (`Actor.K2_DestroyActor` (`self.GetOwner`))))