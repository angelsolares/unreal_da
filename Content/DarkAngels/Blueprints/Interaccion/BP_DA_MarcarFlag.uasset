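; BP_DA_MarcarFlag is an actor that marks a game flag when its linked interactable begins being inspected.
; Every Tick, Vigilar casts Encuadre to BP_DA_Interactuable and compares Inspeccionando with the stored HablandoAntes to detect the rising edge by polling.
; On that edge it sets Hecho and calls MarcarFlag with its Flag on BP_DA_GameState.
; Hecho is never checked here, so each new inspection marks the flag again.
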(event `self.ReceiveTick`
  (params (DeltaSeconds :type "Float (single-precision)"))
  (`self.Vigilar`))

(fn `UserConstructionScript`)

(fn `Vigilar`
  (bind _encuadre (`self.Encuadre`))
  (`/Engine/EditorBlueprintResources/StandardMacros.IsValid` _encuadre
    (:`Is Valid`
      (bind _asbp_da_interactuable (cast `/Game/DarkAngels/Blueprints/Interaccion/BP_DA_Interactuable` _encuadre))
      (bind _inspeccionando (`/Game/DarkAngels/Blueprints/Interaccion/BP_DA_Interactuable.Inspeccionando` _asbp_da_interactuable))
      (if (and _inspeccionando (not (`self.HablandoAntes`)))
        (set `self.Hecho` true)
        (bind _asbp_da_game_state (cast `/Game/DarkAngels/Blueprints/World/BP_DA_GameState` (`GameplayStatics.GetGameState`)))
        (`/Game/DarkAngels/Blueprints/World/BP_DA_GameState.MarcarFlag` _asbp_da_game_state (`self.Flag`)))
      (set `self.HablandoAntes` _inspeccionando))))