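; Interactable actor for DarkAngels that toggles an inspection view, with an optional talking animation and closed-to-open actor swap.
; Interact turns it along the player-to-target yaw, blends the camera to Zona's owner, hides the player and attached actors, and blocks move/look input.
; Interacting again restores idle animation, camera, player and input, but leaves the open state.
; The prompt shows Verbo, or "Aceptar" while inspecting.
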(event `/Game/DynamicCombatSystem/DCS/Blueprints/Interfaces/I_IsInteractable.Interact`
  (params (Caller :type "Actor Object Reference"))
  (bind _returnvalue (`GameplayStatics.GetPlayerController` 0))
  (bind _returnvalue_2 (`GameplayStatics.GetPlayerCharacter` 0))
  (bind _animado (`self.Animado`))
  (bind _cerrado (`self.Cerrado`))
  (bind _abierto (`self.Abierto`))
  (bind _animado_2 (`self.Animado`))
  (bind _returnvalue_3 (`ActorComponent.GetOwner` (`self.Zona`)))
  (if (`self.Inspeccionando`)
    (`/Engine/EditorBlueprintResources/StandardMacros.IsValid` _animado
      (:`Is Valid`
        (`SkeletalMeshComponent.PlayAnimation` (`SkeletalMeshActor.SkeletalMeshComponent` _animado) (`self.AnimReposo`) true))
      (:`Is Not Valid`
        _))
    (`PlayerController.SetViewTargetWithBlend` _returnvalue _returnvalue_2 0.35 "VTBlend_Linear" 0.0 false)
    (`self.SetActorHiddenInGame` _returnvalue_2 false)
    (for _array_element (`self.GetAttachedActors` _returnvalue_2 true true)
      (`self.SetActorHiddenInGame` _array_element false))
    (`Controller.SetIgnoreMoveInput` _returnvalue false)
    (`Controller.SetIgnoreLookInput` _returnvalue false)
    (set `self.Inspeccionando` false)
    (else
      (`self.K2_SetActorRotation` (`KismetMathLibrary.MakeRotator` 0.0 0.0 (.yaw (`KismetMathLibrary.FindLookAtRotation` (`self.K2_GetActorLocation` _returnvalue_2) (`self.K2_GetActorLocation` _returnvalue_3)))))
      (`/Engine/EditorBlueprintResources/StandardMacros.IsValid` _cerrado
        (:`Is Valid`
          (`self.SetActorHiddenInGame` _cerrado true))
        (:`Is Not Valid`
          _))
      (`/Engine/EditorBlueprintResources/StandardMacros.IsValid` _abierto
        (:`Is Valid`
          (`self.SetActorHiddenInGame` _abierto false))
        (:`Is Not Valid`
          _))
      (`/Engine/EditorBlueprintResources/StandardMacros.IsValid` _animado_2
        (:`Is Valid`
          (`SkeletalMeshComponent.PlayAnimation` (`SkeletalMeshActor.SkeletalMeshComponent` _animado_2) (`self.AnimHablar`) true))
        (:`Is Not Valid`
          _))
      (`PlayerController.SetViewTargetWithBlend` _returnvalue _returnvalue_3 0.35 "VTBlend_Linear" 0.0 false)
      (`self.SetActorHiddenInGame` _returnvalue_2 true)
      (for _array_element_2 (`self.GetAttachedActors` _returnvalue_2 true true)
        (`self.SetActorHiddenInGame` _array_element_2 true))
      (`Controller.SetIgnoreMoveInput` _returnvalue true)
      (`Controller.SetIgnoreLookInput` _returnvalue true)
      (set `self.Inspeccionando` true))))

(event `self.ReceiveTick`
  (params (DeltaSeconds :type "Float (single-precision)")))

(fn `GetInteractionMessage`
  (returns (Message :type Name))
  (return (`KismetStringLibrary.Conv_StringToName` (`KismetMathLibrary.SelectString` "Aceptar" (`self.Verbo`) (`self.Inspeccionando`)))))

(fn `UserConstructionScript`)