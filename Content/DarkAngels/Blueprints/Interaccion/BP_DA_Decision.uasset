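; One-time dialogue decision that drives a linked BP_DA_Interactuable (Encuadre) by overwriting its three dialogue lines.
; Tick polls Inspeccionando: when the first inspection ends, it writes the options, hiding the third unless the GameState has FlagOpcion3.
; During a later inspection, keys 1-3 lock in a choice.
; The choice swaps in its response lines from per-option arrays and records its named mark and strength via AnotarMarca on BP_DA_GameState.
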(event `self.ReceiveTick`
  (params (DeltaSeconds :type "Float (single-precision)"))
  (`self.Vigilar`))

(fn `Elegir`
  (params (Opcion :type Integer))
  (bind _returnvalue (- Opcion 1))
  (bind _asbp_da_game_state (cast `/Game/DarkAngels/Blueprints/World/BP_DA_GameState` (`GameplayStatics.GetGameState`)))
  (bind _tiene (`/Game/DarkAngels/Blueprints/World/BP_DA_GameState.TieneFlag` _asbp_da_game_state (`self.FlagOpcion3`)))
  (if (and (== (`self.Elegida`) 0) (or (!= Opcion 3) _tiene))
    (set `self.Elegida` Opcion)
    (set `self.Paso` 2)
    (bind _asbp_da_interactuable (cast `/Game/DarkAngels/Blueprints/Interaccion/BP_DA_Interactuable` (`self.Encuadre`)))
    (set `/Game/DarkAngels/Blueprints/Interaccion/BP_DA_Interactuable.Dialogo1` (`|GetArrayItem` (`self.Rev1`) _returnvalue) _asbp_da_interactuable)
    (set `/Game/DarkAngels/Blueprints/Interaccion/BP_DA_Interactuable.Dialogo2` (`|GetArrayItem` (`self.Rev2`) _returnvalue) _asbp_da_interactuable)
    (set `/Game/DarkAngels/Blueprints/Interaccion/BP_DA_Interactuable.Dialogo3` (`|GetArrayItem` (`self.Rev3`) _returnvalue) _asbp_da_interactuable)
    (`/Game/DarkAngels/Blueprints/World/BP_DA_GameState.AnotarMarca` _asbp_da_game_state (`|GetArrayItem` (`self.Fuerza`) _returnvalue) (`|GetArrayItem` (`self.Marca`) _returnvalue))))

(fn `EscribirOpciones`
  (bind _asbp_da_interactuable (cast `/Game/DarkAngels/Blueprints/Interaccion/BP_DA_Interactuable` (`self.Encuadre`)))
  (bind _asbp_da_game_state (cast `/Game/DarkAngels/Blueprints/World/BP_DA_GameState` (`GameplayStatics.GetGameState`)))
  (set `/Game/DarkAngels/Blueprints/Interaccion/BP_DA_Interactuable.Dialogo1` (`self.Opcion1`) _asbp_da_interactuable)
  (set `/Game/DarkAngels/Blueprints/Interaccion/BP_DA_Interactuable.Dialogo2` (`self.Opcion2`) _asbp_da_interactuable)
  (bind _tiene (`/Game/DarkAngels/Blueprints/World/BP_DA_GameState.TieneFlag` _asbp_da_game_state (`self.FlagOpcion3`)))
  (set `/Game/DarkAngels/Blueprints/Interaccion/BP_DA_Interactuable.Dialogo3` (select `bool` _tiene :`false` "" :`true` (`self.Opcion3`)) _asbp_da_interactuable))

(fn `LeerTeclas`
  (bind _returnvalue (`GameplayStatics.GetPlayerController` 0))
  (if (`PlayerController.WasInputKeyJustPressed` _returnvalue "One")
    (`self.Elegir` 1))
  (if (`PlayerController.WasInputKeyJustPressed` _returnvalue "Two")
    (`self.Elegir` 2))
  (if (`PlayerController.WasInputKeyJustPressed` _returnvalue "Three")
    (`self.Elegir` 3)))

(fn `UserConstructionScript`)

(fn `Vigilar`
  (bind _encuadre (`self.Encuadre`))
  (`/Engine/EditorBlueprintResources/StandardMacros.IsValid` _encuadre
    (:`Is Valid`
      (bind _asbp_da_interactuable (cast `/Game/DarkAngels/Blueprints/Interaccion/BP_DA_Interactuable` _encuadre))
      (bind _inspeccionando (`/Game/DarkAngels/Blueprints/Interaccion/BP_DA_Interactuable.Inspeccionando` _asbp_da_interactuable))
      (if (and (`self.HablandoAntes`) (not _inspeccionando))
        (if (== (`self.Paso`) 0)
          (set `self.Paso` 1)
          (`self.EscribirOpciones`)))
      (if (and _inspeccionando (== (`self.Paso`) 1))
        (if (== (`self.Elegida`) 0)
          (`self.LeerTeclas`)))
      (set `self.HablandoAntes` _inspeccionando))))