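; BP_DA_GabrielHeraldo drives the Gabriel herald, an inspectable figure that watches the player and can fly away after being inspected.
; On Tick, it smoothly turns the Animado actor's yaw toward the player within a radius.
; Inspection sets HaHablado; once it ends, SeVaAlHablar triggers departure.
; Departure offsets the actor forward and vertically over a timed flight without sweeping, then hides it rather than destroying it.
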(event `self.ReceiveTick`
  (params (DeltaSeconds :type "Float (single-precision)"))
  (bind _animado (`self.Animado`))
  (bind _returnvalue (`self.K2_GetActorLocation` (`GameplayStatics.GetPlayerCharacter` 0)))
  (bind _returnvalue_2 (`self.K2_GetActorLocation` _animado))
  (`parent.ReceiveTick` DeltaSeconds)
  (if (`KismetSystemLibrary.IsValid` (`self.Animado`))
    (if (`self.Yendose`)
      (if (> (- (`KismetSystemLibrary.GetGameTimeInSeconds`) (`self.Partida`)) (`self.SegundosVuelo`))
        (`self.SetActorHiddenInGame` (`self.Animado`) true)
        (else
          (`self.K2_AddActorWorldOffset` (`self.Animado`) (* (+ (* (`self.GetActorForwardVector` (`self.Animado`)) (`self.AvanceVuelo`)) (`KismetMathLibrary.MakeVector` 0.0 0.0 (`self.AlturaVuelo`))) (/ DeltaSeconds (`self.SegundosVuelo`))) false false)))
      (elif (`self.Inspeccionando`)
        (set `self.HaHablado` true)
        (elif (and (`self.HaHablado`) (`self.SeVaAlHablar`))
          (set `self.Yendose` true)
          (set `self.Partida` (`KismetSystemLibrary.GetGameTimeInSeconds`))
          (elif (< (`KismetMathLibrary.Vector_Distance` _returnvalue_2 _returnvalue) (`self.RadioMirada`))
            (`self.K2_SetActorRotation` (`self.Animado`) (`KismetMathLibrary.RInterpTo` (`self.K2_GetActorRotation` _animado) (`KismetMathLibrary.MakeRotator` 0.0 0.0 (.yaw (`KismetMathLibrary.FindLookAtRotation` _returnvalue_2 _returnvalue))) DeltaSeconds (`self.VelocidadMirada`)) false)))))))

(fn `UserConstructionScript`
  (`parent.UserConstructionScript`))